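; Master Blueprint for an interactive double door that opens and closes by swinging or sliding when the player presses F inside its trigger.
; The construction script makes slide and swing mutually exclusive based on IsSwingType.
; Timelines, rate-scaled by AnimationTime, play or reverse to mirror rotation or offset across two pivots.
; DoorInteract plays open or close sounds and ignores input while animating.
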(event `self.ReceiveBeginPlay`
  (bind _t_doorswing (`self.T_DoorSwing`))
  (bind _t_doorslide (`self.T_DoorSlide`))
  (bind _returnvalue (`TimelineComponent.GetTimelineLength` _t_doorslide))
  (bind _returnvalue_2 (`TimelineComponent.GetTimelineLength` _t_doorswing))
  (`|ExecutionSequence`
    (:`then_0`
      (set `self.SourcePosition` (`SceneComponent.RelativeLocation` (`self.Pivot`)))
      (`|ExecutionSequence`
        (:`then_0`
          (`TimelineComponent.SetPlayRate` _t_doorswing (/ _returnvalue_2 (* _returnvalue_2 (`self.AnimationTime`)))))
        (:`then_1`
          (`TimelineComponent.SetPlayRate` _t_doorslide (/ _returnvalue (* _returnvalue (`self.AnimationTime`)))))))
    (:`then_1`
      (set `self.SourcePosition2` (`SceneComponent.RelativeLocation` (`self.Pivot2`))))))

(event `self.Trigger.OnComponentBeginOverlap`
  (params (OverlappedComponent :type "PrimitiveComponent Object Reference") (OtherActor :type "Actor Object Reference") (OtherComp :type "PrimitiveComponent Object Reference") (OtherBodyIndex :type Integer) (bFromSweep :type Boolean) (SweepResult :type "HitResult Structure (by ref)"))
  (set `self.IsInRange` (== OtherActor (`GameplayStatics.GetPlayerPawn` 0))))

(event `self.Trigger.OnComponentEndOverlap`
  (params (OverlappedComponent :type "PrimitiveComponent Object Reference") (OtherActor :type "Actor Object Reference") (OtherComp :type "PrimitiveComponent Object Reference") (OtherBodyIndex :type Integer))
  (if (== OtherActor (`GameplayStatics.GetPlayerPawn` 0))
    (set `self.IsInRange` false)))

(event `Key|F` :consume false
  (params (Key :type "Key Structure"))
  (:`Pressed`
    (if (`self.IsInRange`)
      (`self.DoorInteract`))))

(event `DoorInteract`
  (bind _sourceposition (`self.SourcePosition`))
  (bind _sourceposition2 (`self.SourcePosition2`))
  (if (not (`self.IsAnimating`))
    (`|ExecutionSequence`
      (:`then_0`
        (if (`self.IsSwingType`)
          (`self.PlaySound`)
          (if (`self.IsOpen`)
            (bind (_direction _alpha) (`Timeline|T_DoorSwing` :!via `Reverse` :!label _label)
              (:`Update`
                (`|ExecutionSequence`
                  (:`then_0`
                    (`SceneComponent.K2_SetRelativeRotation` (`self.Pivot`) (`KismetMathLibrary.RLerp` (struct) (`self.TargetRotation`) _alpha true) false false))
                  (:`then_1`
                    (`SceneComponent.K2_SetRelativeRotation` (`self.Pivot2`) (`KismetMathLibrary.RLerp` (struct) (`KismetMathLibrary.NegateRotator` (`self.TargetRotation`)) _alpha true) false false))))
              (:`Finished`
                (set `self.IsOpen` (not (`self.IsOpen`)))
                (set `self.IsAnimating` false)))
            (else
              (goto _label)))))
      (:`then_1`
        (if (`self.IsSlideType`)
          (`self.PlaySound`)
          (if (`self.IsOpen`)
            (bind (_direction_2 _alpha_2) (`Timeline|T_DoorSlide` :!via `Reverse` :!label _label_2)
              (:`Update`
                (`|ExecutionSequence`
                  (:`then_0`
                    (`SceneComponent.K2_SetRelativeLocation` (`self.Pivot`) (`KismetMathLibrary.VLerp` _sourceposition (+ _sourceposition (`self.TargetPosition`)) _alpha_2) false false))
                  (:`then_1`
                    (`SceneComponent.K2_SetRelativeLocation` (`self.Pivot2`) (`KismetMathLibrary.VLerp` _sourceposition2 (+ _sourceposition2 (`KismetMathLibrary.NegateVector` (`self.TargetPosition`))) _alpha_2) false false))))
              (:`Finished`
                (set `self.IsOpen` (not (`self.IsOpen`)))
                (set `self.IsAnimating` false)))
            (else
              (goto _label_2)))))
      (:`then_2`
        (set `self.IsAnimating` true)))))

(event `PlaySound`
  (bind _returnvalue (`SceneComponent.K2_GetComponentLocation` (`self.Pivot`)))
  (if (`self.IsOpen`)
    (`GameplayStatics.PlaySoundAtLocation` (`self.SC_Close`) _returnvalue (struct) 1.0 1.0 0.0 null null null)
    (else
      (`GameplayStatics.PlaySoundAtLocation` (`self.SC_Open`) _returnvalue (struct) 1.0 1.0 0.0 null null null))))

(fn `UserConstructionScript`
  (if (`self.IsSwingType`)
    (set `self.IsSlideType` false)
    (else
      (set `self.IsSlideType` true))))