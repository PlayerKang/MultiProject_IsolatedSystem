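; BP_BasementDoor is an interactable door that moves the multiplayer session to the InGame_BaseMent level.
; Its Box overlap sets ReadyToBasement on each BP_Survivor entering and clears it on exit.
; InterectionInput requires an equipped SecurityCard in the user's BPC_InventorySystem, then checks every survivor is ready, printing a message when either check fails.
; When both pass, only the authority runs servertravel through a console command.
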(event `/Game/WorkByKang/BluePrint/Interection/BPI_Interection.InterectionInput`
  (params (Character :type "Actor Object Reference"))
  (bind _equipeditem (`/Game/WorkByKang/BluePrint/Inventory/BPC_InventorySystem.EquipedItem` (`self.GetComponentByClass` Character "/Game/WorkByKang/BluePrint/Inventory/BPC_InventorySystem.BPC_InventorySystem_C"))
    (:`then`
      (if (== (`/Game/Item/Blueprints/BP_ItemParent.ItemRowName` _equipeditem) "SecurityCard")
        (bind _outactors (`GameplayStatics.GetAllActorsOfClass` "/Game/MainBluePrints/BP_Survivor.BP_Survivor_C"))
        (for _array_element _outactors
          (if (`/Game/MainBluePrints/BP_Survivor.ReadyToBasement` _array_element)
            (set `self.Is All Player Ready?` true)
            (else
              (set `self.Is All Player Ready?` false)
              (`KismetSystemLibrary.PrintString` "Need All Player")
              (break))))
        (if (`self.Is All Player Ready?`)
          (`/Engine/EditorBlueprintResources/ActorMacros.Switch Has Authority`
            (:`Authority`
              (`KismetSystemLibrary.ExecuteConsoleCommand` "servertravel InGame_BaseMent" null))))
        (else
          (`KismetSystemLibrary.PrintString` "Need Security Card" :!label _label))))
    (:`else`
      (goto _label))))

(event `self.Box.OnComponentBeginOverlap`
  (params (OverlappedComponent :type "PrimitiveComponent Object Reference") (OtherActor :type "Actor Object Reference") (OtherComp :type "PrimitiveComponent Object Reference") (OtherBodyIndex :type Integer) (bFromSweep :type Boolean) (SweepResult :type "HitResult Structure (by ref)"))
  (bind _asbp_survivor (cast `/Game/MainBluePrints/BP_Survivor` OtherActor))
  (set `/Game/MainBluePrints/BP_Survivor.ReadyToBasement` true _asbp_survivor))

(event `self.Box.OnComponentEndOverlap`
  (params (OverlappedComponent :type "PrimitiveComponent Object Reference") (OtherActor :type "Actor Object Reference") (OtherComp :type "PrimitiveComponent Object Reference") (OtherBodyIndex :type Integer))
  (bind _asbp_survivor (cast `/Game/MainBluePrints/BP_Survivor` OtherActor))
  (set `/Game/MainBluePrints/BP_Survivor.ReadyToBasement` false _asbp_survivor))

(fn `UserConstructionScript`)