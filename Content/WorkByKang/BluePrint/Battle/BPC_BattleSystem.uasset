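; BPC_BattleSystem is a component on BP_Survivor that handles first-person combat input: bat attacks and throwing the held item.
; Left and right clicks play separate bat attack montages, while a held right click turns left click into a throw.
; Throwing spawns the item at the camera, applies a forward impulse scaled by clamped hold time, then notifies the inventory component.
; Attack and Parry are empty stubs, and hold animations are print placeholders.
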(event `self.ReceiveBeginPlay`
  ;[1 1 1] Set My Character
  (bind _asbp_survivor (cast `/Game/MainBluePrints/BP_Survivor` (`self.GetOwner`)))
  (set `self.MyCharacter` _asbp_survivor))

(event `EnhancedInput|/Game/Input/Attack/IA_LeftClick`
  (params (ActionValue :type Boolean) (ElapsedSeconds :type "Float (double-precision)") (TriggeredSeconds :type "Float (double-precision)") (InputAction :type "InputAction Object Reference" :default "/Game/Input/Attack/IA_LeftClick.IA_LeftClick"))
  (:`Started`
    (if (and (`self.IsRightClickPressed`) (`self.IsHoldProgressed`))
      (`self.ThrowItem`)
      (set `self.IsWeaponThrowed` true)
      (else
        (`|PlayMontage` (`Character_Survivor.FPSMesh` (`self.MyCharacter`)) "/Game/ArmsMeleeFPSAndBonusTemplate/MeleePACK/bat/Anims/Anim_Bat_Attack_02_Montage.Anim_Bat_Attack_02_Montage"
          (:`then`
            (`self.Attack`)))))))

(event `EnhancedInput|/Game/Input/Attack/IA_RightClick`
  (params (ActionValue :type Boolean) (ElapsedSeconds :type "Float (double-precision)") (TriggeredSeconds :type "Float (double-precision)") (InputAction :type "InputAction Object Reference" :default "/Game/Input/Attack/IA_RightClick.IA_RightClick"))
  (:`Triggered`
    (set `self.RightClickHoldTime` ElapsedSeconds))
  (:`Started`
    (set `self.IsRightClickPressed` true))
  (:`Completed`
    (set `self.IsRightClickPressed` false)
    (if (`self.IsHoldProgressed`)
      (set `self.IsHoldProgressed` false)
      (if (not (`self.IsWeaponThrowed`))
        (`KismetSystemLibrary.PrintString` "weapon down anim"))
      (else
        (`|PlayMontage` (`Character_Survivor.FPSMesh` (`self.MyCharacter`)) "/Game/ArmsMeleeFPSAndBonusTemplate/MeleePACK/bat/Anims/Anim_Bat_Attack_01_Montage.Anim_Bat_Attack_01_Montage")))))

(event `EnhancedInput|/Game/Input/Attack/IA_RightClickHold`
  (params (ActionValue :type Boolean) (ElapsedSeconds :type "Float (double-precision)") (TriggeredSeconds :type "Float (double-precision)") (InputAction :type "InputAction Object Reference" :default "/Game/Input/Attack/IA_RightClickHold.IA_RightClickHold"))
  (:`Triggered`
    (`KismetSystemLibrary.PrintString` "hold anim")
    (set `self.IsHoldProgressed` true)))

(fn `Attack`)

(fn `Parry`)

(fn `ThrowItem`
  (bind _mycharacter (`self.MyCharacter`))
  (bind (_returnvalue_location _returnvalue_rotation) (`KismetMathLibrary.BreakTransform` (`SceneComponent.K2_GetComponentToWorld` (`/Game/MainBluePrints/BP_Survivor.CameraFrontPoint` _mycharacter))))
  (bind (_handonitemname _handonitemname_2) (`/Game/WorkByKang/BluePrint/Inventory/BPC_InventorySystem.HandOnItemName` (`/Game/MainBluePrints/BP_Survivor.BPC_InventorySystem` _mycharacter)))
  (bind _returnvalue (`|SpawnActorFromClass` "/Game/Item/Blueprints/BP_All_ItemSpawner.BP_All_ItemSpawner_C" (`KismetMathLibrary.MakeTransform` _returnvalue_location _returnvalue_rotation (.scale (break `/Game/Item/S_All_Item` _handonitemname_2))) "Undefined" "OverrideRootScale" null _handonitemname null))
  (`PrimitiveComponent.AddImpulse` (`/Game/Item/Blueprints/BP_All_ItemSpawner.Item` _returnvalue) (* (`KismetMathLibrary.GetForwardVector` _returnvalue_rotation) (`KismetMathLibrary.FClamp` (* (`self.RightClickHoldTime`) 500.0) 0.0 2000.0)) "None" false)
  (`/Game/WorkByKang/BluePrint/Inventory/BPC_InventorySystem.ThrowItemFromInventory` (`/Game/MainBluePrints/BP_Survivor.BPC_InventorySystem` (`self.MyCharacter`))))