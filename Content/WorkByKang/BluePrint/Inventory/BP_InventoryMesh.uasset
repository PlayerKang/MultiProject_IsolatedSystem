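; BP_InventoryMesh is an inventory display that represents item stock with meshes and links to the player survivor's BPCInventorySystem.
; SetItemVisibilityByStock shows zero to five meshes by count.
; SetInventoryMesh calls it per MaxStock without arguments; the per-item mapping, padded with JunkMesh, is disconnected.
; SendAndCloseInventory equips the item named by the object's underscore prefix and closes the inventory, but its EventGraph call is unwired.
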(event `self.ReceiveBeginPlay`
  (bind _asbp_survivor (cast `/Game/MainBluePrints/BP_Survivor` (`GameplayStatics.GetPlayerPawn` 0)))
  (set `self.Inventory System` (`/Game/MainBluePrints/BP_Survivor.BPC_InventorySystem` _asbp_survivor)))

(fn `SendAndCloseInventory`
  (params (Object :type "Object Object Reference"))
  (bind _inventory_system (`self.Inventory System`))
  (`/Game/WorkByKang/BluePrint/Inventory/BPC_InventorySystem.EquipOnHand` _inventory_system (`KismetStringLibrary.Conv_StringToName` (`KismetStringLibrary.Split` (`KismetSystemLibrary.GetObjectName` Object) "_")))
  (`/Game/WorkByKang/BluePrint/Inventory/BPC_InventorySystem.CloseInventory` _inventory_system))

(fn `SetInventoryMesh`
  (for _array_element (`self.Stocks`)
    (for _ (range (`.MaxStock_9_EE014A7C4765C53C72A74FB016CB6E49` (break `/Game/Item/S_All_Item` _array_element)))
      (`self.SetItemVisibilityByStock` null))))

(fn `SetItemVisibilityByStock`
  (params (`0` :type "StaticMeshComponent Object Reference") (`1` :type "StaticMeshComponent Object Reference") (`2` :type "StaticMeshComponent Object Reference") (`3` :type "StaticMeshComponent Object Reference") (`4` :type "StaticMeshComponent Object Reference") (NowStock :type Integer))
  (switch `int` NowStock
    (:`0`
      (`SceneComponent.SetVisibility` `0` false false)
      (`SceneComponent.SetVisibility` `1` false false)
      (`SceneComponent.SetVisibility` `2` false false)
      (`SceneComponent.SetVisibility` `3` false false)
      (`SceneComponent.SetVisibility` `4` false false))
    (:`1`
      (`SceneComponent.SetVisibility` `0` true false)
      (`SceneComponent.SetVisibility` `2` false false)
      (`SceneComponent.SetVisibility` `3` false false)
      (`SceneComponent.SetVisibility` `4` false false)
      (`SceneComponent.SetVisibility` `1` false false))
    (:`2`
      (`SceneComponent.SetVisibility` `0` true false)
      (`SceneComponent.SetVisibility` `1` true false)
      (`SceneComponent.SetVisibility` `2` false false)
      (`SceneComponent.SetVisibility` `3` false false)
      (`SceneComponent.SetVisibility` `4` false false))
    (:`3`
      (`SceneComponent.SetVisibility` `0` true false)
      (`SceneComponent.SetVisibility` `1` true false)
      (`SceneComponent.SetVisibility` `2` true false)
      (`SceneComponent.SetVisibility` `3` false false)
      (`SceneComponent.SetVisibility` `4` false false))
    (:`4`
      (`SceneComponent.SetVisibility` `0` true false)
      (`SceneComponent.SetVisibility` `1` true false)
      (`SceneComponent.SetVisibility` `2` true false)
      (`SceneComponent.SetVisibility` `3` true false)
      (`SceneComponent.SetVisibility` `4` false false))
    (:`5`
      (`SceneComponent.SetVisibility` `0` true false)
      (`SceneComponent.SetVisibility` `1` true false)
      (`SceneComponent.SetVisibility` `2` true false)
      (`SceneComponent.SetVisibility` `3` true false)
      (`SceneComponent.SetVisibility` `4` true false))))

(fn `UserConstructionScript`)