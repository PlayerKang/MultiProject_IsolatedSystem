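; Inventory component for BP_Survivor that handles item stock, quick slots and the item held in hand.
; DT_Item seeds the stock array; pickups raise counts, fill a free quick slot and destroy the world actor through REQ/RES events.
; Wheel and number inputs spawn the selected item on the FPS mesh's hand socket and set its anim type, dropping non-inventory items.
; Tab toggles a spawned 3D inventory mesh, enabling the cursor and locking look and movement.
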(event `self.ReceiveBeginPlay`
  (`|ExecutionSequence`
    (:`then_0`
      ;[1 1 1] Set My Character
      (bind _asbp_survivor (cast `/Game/MainBluePrints/BP_Survivor` (`self.GetOwner`)))
      (set `self.MyCharacter` _asbp_survivor))
    (:`then_1`
      ;[1 1 1] Set Item Array
      (bind _outrownames (`DataTableFunctionLibrary.GetDataTableRowNames` "/Game/Item/DT_Item.DT_Item"))
      (for _array_element _outrownames
        (bind _returnvalue (`|GetDataTableRow` "/Game/Item/DT_Item.DT_Item" _array_element)
          (:`then`
            (`KismetArrayLibrary.Array_AddUnique` (`self.Stocks`) _returnvalue)))))
    (:`then_2`
      (for (_array_element_2 _array_index) (`self.Stocks`)
        (bind _structout (setmembers `/Game/Item/S_All_Item` :`StructRef` _array_element_2 :`NowStock` 0))
        (`KismetArrayLibrary.Array_Set` (`self.Stocks`) _array_index _structout)))
    (:`then_3`
      ;[1 1 1] QuickSlot Size
      (`KismetArrayLibrary.Array_Resize` (`self.QuickSlots`) 5))))

(event `EnhancedInput|/Game/Input/Interface/IA_Tab_Inventory`
  (params (ActionValue :type Boolean) (ElapsedSeconds :type "Float (double-precision)") (TriggeredSeconds :type "Float (double-precision)") (InputAction :type "InputAction Object Reference" :default "/Game/Input/Interface/IA_Tab_Inventory.IA_Tab_Inventory"))
  ;[1 1 1] Inventory Input
  (:`Started`
    (if (`self.IsInventoryOpen`)
      (`self.CloseInventory`)
      (else
        (`self.SetInventoryMeshData`)
        (`|PlayMontage` (`Character_Survivor.FPSMesh` (`self.MyCharacter`))
          (:`then`
            (`self.OpenInventory`)))))))

(event `EnhancedInput|/Game/Input/Interface/IA_MouseWheel`
  (params (ActionValue :type "Float (double-precision)") (ElapsedSeconds :type "Float (double-precision)") (TriggeredSeconds :type "Float (double-precision)") (InputAction :type "InputAction Object Reference" :default "/Game/Input/Interface/IA_MouseWheel.IA_MouseWheel"))
  (bind _returnvalue (+ (`KismetMathLibrary.FTrunc` ActionValue) (`self.EquippedSlot`)))
  ;[1 1 1] QuickSlot Control
  (:`Started`
    (if (`KismetArrayLibrary.Array_IsValidIndex` (`self.QuickSlots`) _returnvalue)
      (set `self.EquippedSlot` _returnvalue)
      (elif (< _returnvalue 0)
        (set `self.EquippedSlot` (`KismetArrayLibrary.Array_LastIndex` (`self.QuickSlots`)))
        (else
          (set `self.EquippedSlot` 0))))
    (bind _output_get (set `self.HandOnItemName` (`self.GetItemNameByQuickSlot`)))
    (`self.EquipOnHand` _output_get)))

(event `EnhancedInput|/Game/Input/Interface/IA_QuickSlot1`
  (params (ActionValue :type Boolean) (ElapsedSeconds :type "Float (double-precision)") (TriggeredSeconds :type "Float (double-precision)") (InputAction :type "InputAction Object Reference" :default "/Game/Input/Interface/IA_QuickSlot1.IA_QuickSlot1"))
  ;[1 1 1] QuickSlot Control
  (:`Started`
    (if (== (`self.EquippedSlot`) 1)
      (set `self.EquippedSlot` 0 :!label _label)
      (bind _output_get (set `self.HandOnItemName` "None"))
      (`self.EquipOnHand` _output_get)
      (else
        (set `self.EquippedSlot` 1)
        (bind _output_get_2 (set `self.HandOnItemName` (`self.GetItemNameByQuickSlot`) :!label _label_2))
        (`self.EquipOnHand` _output_get_2)))))

(event `EnhancedInput|/Game/Input/Interface/IA_QuickSlot2`
  (params (ActionValue :type Boolean) (ElapsedSeconds :type "Float (double-precision)") (TriggeredSeconds :type "Float (double-precision)") (InputAction :type "InputAction Object Reference" :default "/Game/Input/Interface/IA_QuickSlot2.IA_QuickSlot2"))
  ;[1 1 1] QuickSlot Control
  (:`Started`
    (if (== (`self.EquippedSlot`) 2)
      (goto _label)
      (else
        (set `self.EquippedSlot` 2)
        (goto _label_2)))))

(event `EnhancedInput|/Game/Input/Interface/IA_QuickSlot3`
  (params (ActionValue :type Boolean) (ElapsedSeconds :type "Float (double-precision)") (TriggeredSeconds :type "Float (double-precision)") (InputAction :type "InputAction Object Reference" :default "/Game/Input/Interface/IA_QuickSlot3.IA_QuickSlot3"))
  ;[1 1 1] QuickSlot Control
  (:`Started`
    (if (== (`self.EquippedSlot`) 3)
      (goto _label)
      (else
        (set `self.EquippedSlot` 3)
        (goto _label_2)))))

(event `EnhancedInput|/Game/Input/Interface/IA_QuickSlot4`
  (params (ActionValue :type Boolean) (ElapsedSeconds :type "Float (double-precision)") (TriggeredSeconds :type "Float (double-precision)") (InputAction :type "InputAction Object Reference" :default "/Game/Input/Interface/IA_QuickSlot4.IA_QuickSlot4"))
  ;[1 1 1] QuickSlot Control
  (:`Started`
    (if (== (`self.EquippedSlot`) 4)
      (goto _label)
      (else
        (set `self.EquippedSlot` 4)
        (goto _label_2)))))

(event `REQ Destroy Item`
  (params (`Hit Item` :type "/Game/Item/Blueprints/BP_ItemParent Object Reference"))
  (`self.RES Destroy Item` `Hit Item`))

(event `RES Destroy Item`
  (params (`Hit Item` :type "/Game/Item/Blueprints/BP_ItemParent Object Reference"))
  (`Actor.K2_DestroyActor` `Hit Item`))

(fn `AddItem`
  (params (ItemRowName :type Name))
  (returns (Result :type Boolean))
  (for (_array_element _array_index) (`self.Stocks`)
    (bind (_itemtype _name _maxstock _nowstock) (break `/Game/Item/S_All_Item` _array_element))
    (if (== _name ItemRowName)
      (bind _returnvalue (+ _nowstock 1))
      (if (>= _maxstock _returnvalue)
        (bind _structout (setmembers `/Game/Item/S_All_Item` :`StructRef` _array_element :`NowStock` _returnvalue))
        (`KismetArrayLibrary.Array_Set` (`self.Stocks`) _array_index _structout)
        (`KismetSystemLibrary.PrintString` (`KismetStringLibrary.Conv_NameToString` _name) true true (struct :`G` 0.572917 :`B` 0.070918 :`A` 1.0) 10.0)
        (return true)
        (else
          (return false))))))

(fn `AddQuikslot`
  (params (ItemName :type Name) (SlotNumber :type Integer))
  (bind _returnvalue (`|GetDataTableRow` "/Game/Item/DT_Item.DT_Item" ItemName)
    (:`then`
      (`KismetArrayLibrary.Array_Set` (`self.QuickSlots`) SlotNumber _returnvalue))))

(fn `ClickCombineItem`
  (params (ItemName1 :type Name) (ItemName2 :type Name))
  (`self.AddItem` "None")
  (`self.RemoveItem` ItemName1)
  (`self.RemoveItem` ItemName2))

(fn `CloseInventory`
  (bind _returnvalue (`GameplayStatics.GetPlayerController` 0))
  (`Actor.K2_DestroyActor` (`self.SpawnedInventory`))
  (set `self.IsInventoryOpen` false)
  (set `PlayerController.bShowMouseCursor` false _returnvalue)
  (set `PlayerController.bEnableClickEvents` false _returnvalue)
  (set `PlayerController.bEnableMouseOverEvents` false _returnvalue)
  (`Controller.ResetIgnoreLookInput` _returnvalue)
  (`CharacterMovementComponent.SetMovementMode` (`Character.CharacterMovement` (`self.MyCharacter`)) "MOVE_Walking" 0))

(fn `EmptyQuickSlot`
  (params (SlotNumber :type Integer))
  (`KismetArrayLibrary.Array_Set` (`self.QuickSlots`) SlotNumber))

(fn `EquipOnHand`
  (params (ItemName :type Name))
  (returns (bResult :type Boolean))
  (bind _returnvalue (`|GetDataTableRow` "/Game/Item/DT_Item.DT_Item" ItemName)
    (:`then`
      (`|ExecutionSequence`
        (:`then_0`
          (bind _bresult (`self.InventoryEquipableCheckAndDropItem`))
          (if _bresult
            (`self.ResetHand`)
            (else
              (`KismetSystemLibrary.PrintString` "spawnfail"))))
        (:`then_1`
          (bind _returnvalue_2 (`|SpawnActorFromClass` (`.BP_47_757DA67542F38347E47E3D9A8BD1682F` (break `/Game/Item/S_All_Item` _returnvalue)) (`.HandSizeTransform_30_9FEC9A164918743D9DE3E39204EF5BEC` (break `/Game/Item/S_All_Item` _returnvalue)) "AlwaysSpawn" "OverrideRootScale" null (`.Name_20_8969098149D6282D7AF70AB804D4FB00` (break `/Game/Item/S_All_Item` _returnvalue)) "NewEnumerator2" null))
          (bind _output_get (set `self.EquipedItem` _returnvalue_2))
          (bind _item (`/Game/Item/Blueprints/BP_ItemParent.Item` _output_get))
          (`/Engine/EditorBlueprintResources/StandardMacros.IsValid` _item
            (:`Is Valid`
              (`PrimitiveComponent.SetSimulatePhysics` _item false)
              (`SceneComponent.K2_AttachToComponent` _item (`Character_Survivor.FPSMesh` (`self.MyCharacter`)) "hand_socket" "KeepRelative" "KeepRelative" "KeepWorld" true))
            (:`Is Not Valid`
              (bind _asbp_body_part (cast `/Game/WorkByKang/Zombies/BodyPart/BP_BodyPart` _output_get))
              (bind _skeletalmesh (`/Game/WorkByKang/Zombies/BodyPart/BP_BodyPart.SkeletalMesh` _asbp_body_part))
              (`PrimitiveComponent.SetSimulatePhysics` _skeletalmesh false)
              (`SceneComponent.K2_AttachToComponent` _skeletalmesh (`Character_Survivor.FPSMesh` (`self.MyCharacter`)) "hand_socket" "KeepRelative" "KeepRelative" "KeepWorld" true)))
          (set `self.HandOnItemName` (`.Name_20_8969098149D6282D7AF70AB804D4FB00` (break `/Game/Item/S_All_Item` _returnvalue)))
          (bind _asbpa_survivor (cast `/Game/Animations/BPA_Survivor` (`SkeletalMeshComponent.GetAnimInstance` (`Character_Survivor.FPSMesh` (`self.MyCharacter`)))))
          (set `/Game/Animations/BPA_Survivor.WeaponBaseType` (`.BaseAnimType_40_CE282F5F4966AD658AA73DBBC032AB02` (break `/Game/Item/S_All_Item` _returnvalue)) _asbpa_survivor)
          (return true))))
    (:`RowNotFound`
      (bind _bresult_2 (`self.InventoryEquipableCheckAndDropItem`))
      (if _bresult_2
        (`self.ResetHand`)
        (return true)))))

(fn `GetItemNameByQuickSlot`
  (returns (QuickSlotItemName :type Name))
  (return (`.Name_20_8969098149D6282D7AF70AB804D4FB00` (break `/Game/Item/S_All_Item` (`|GetArrayItem` (`self.QuickSlots`) (`self.EquippedSlot`))))))

(fn `InventoryEquipableCheckAndDropItem`
  (returns (bResult :type Boolean))
  (bind _equipeditem (`self.EquipedItem`))
  (bind (_returnvalue_location _returnvalue_rotation) (`KismetMathLibrary.BreakTransform` (`SceneComponent.K2_GetComponentToWorld` (`/Game/MainBluePrints/BP_Survivor.CameraFrontPoint` (`self.MyCharacter`)))))
  (`/Engine/EditorBlueprintResources/StandardMacros.IsValid` _equipeditem
    (:`Is Valid`
      (bind _returnvalue (`|GetDataTableRow` "/Game/Item/DT_Item.DT_Item" (`/Game/Item/Blueprints/BP_ItemParent.ItemRowName` _equipeditem))
        (:`then`
          (bind (_itemtype _name _maxstock _nowstock _mesh _handsizetransform _baseanimtype _mass _bp _canequiponinventory) (break `/Game/Item/S_All_Item` _returnvalue))
          (if (not _canequiponinventory)
            (`|SpawnActorFromClass` _bp (`KismetMathLibrary.MakeTransform` _returnvalue_location _returnvalue_rotation (.scale _handsizetransform)) "AlwaysSpawn" "OverrideRootScale" null _name "NewEnumerator2" null))
          (return true))))))

(fn `OpenInventory`
  (bind _returnvalue (`GameplayStatics.GetPlayerController` 0))
  (bind _asbp_survivor (cast `/Game/MainBluePrints/BP_Survivor` (`GameplayStatics.GetPlayerPawn` 0)))
  (bind (_returnvalue_location _returnvalue_rotation) (`KismetMathLibrary.BreakTransform` (`SceneComponent.K2_GetComponentToWorld` (`/Game/MainBluePrints/BP_Survivor.InventoryPoint` _asbp_survivor))))
  (bind _returnvalue_2 (`|SpawnActorFromClass` "/Game/WorkByKang/BluePrint/Inventory/BP_InventoryMesh.BP_InventoryMesh_C" (`KismetMathLibrary.MakeTransform` _returnvalue_location _returnvalue_rotation) "Undefined" "OverrideRootScale" null (`self.ItemMeshData`) null))
  (bind _output_get (set `self.SpawnedInventory` _returnvalue_2))
  (`/Game/WorkByKang/BluePrint/Inventory/BP_InventoryMesh.SetInventoryMesh` _output_get)
  (set `self.IsInventoryOpen` true)
  (set `PlayerController.bShowMouseCursor` true _returnvalue)
  (set `PlayerController.bEnableClickEvents` true _returnvalue)
  (set `PlayerController.bEnableMouseOverEvents` true _returnvalue)
  (`Controller.SetIgnoreLookInput` _returnvalue true)
  (`CharacterMovementComponent.SetMovementMode` (`Character.CharacterMovement` (`self.MyCharacter`)) "MOVE_None" 0))

(fn `Pick Up Item`
  (params (HitItem :type "/Game/Item/Blueprints/BP_ItemParent Object Reference"))
  (bind _itemrowname (`/Game/Item/Blueprints/BP_ItemParent.ItemRowName` HitItem))
  (`|GetDataTableRow` "/Game/Item/DT_Item.DT_Item" _itemrowname
    (:`then`
      (bind _result (`self.AddItem` _itemrowname))
      (if _result
        (`|ExecutionSequence`
          (:`then_0`
            (`self.EquipOnHand` _itemrowname)
            (for (_array_element _array_index) (`self.QuickSlots`)
              (if (and (== (`.Name_20_8969098149D6282D7AF70AB804D4FB00` (break `/Game/Item/S_All_Item` _array_element)) "None") (!= _array_index 0))
                (`self.AddQuikslot` _itemrowname _array_index)
                (break))))
          (:`then_1`
            (`self.REQ Destroy Item` HitItem)))))))

(fn `PickUpTemporarilyItem`
  (params (`타깃` :type "/Game/Item/Blueprints/BP_ItemParent Object Reference"))
  (bind _itemrowname (`/Game/Item/Blueprints/BP_ItemParent.ItemRowName` `타깃`))
  (`KismetSystemLibrary.PrintString` (`KismetStringLibrary.Conv_NameToString` _itemrowname))
  (`|GetDataTableRow` "/Game/Item/DT_Item.DT_Item" _itemrowname
    (:`then`
      (`|ExecutionSequence`
        (:`then_0`
          (`self.EquipOnHand` _itemrowname))
        (:`then_1`
          (`self.REQ Destroy Item` `타깃`))))))

(fn `RemoveItem`
  (params (ItemName :type Name))
  (returns (Result :type Boolean) (RemainStock :type Integer))
  (for (_array_element _array_index) (`self.Stocks`)
    (bind (_itemtype _name _maxstock _nowstock) (break `/Game/Item/S_All_Item` _array_element))
    (if (== _name ItemName)
      (bind _returnvalue (- _nowstock 1))
      (if (>= _returnvalue 0)
        (bind _structout (setmembers `/Game/Item/S_All_Item` :`StructRef` _array_element :`NowStock` _returnvalue))
        (`KismetArrayLibrary.Array_Set` (`self.Stocks`) _array_index _structout)
        (`KismetSystemLibrary.PrintString` (`KismetStringLibrary.Conv_NameToString` _name) true true (struct :`R` 0.604167 :`B` 0.04346 :`A` 1.0) 10.0)
        (return true _nowstock)
        (else
          (`KismetSystemLibrary.PrintString` "No Item" true true (struct :`R` 0.604167 :`B` 0.04346 :`A` 1.0) 10.0)
          (return false 0))))))

(fn `ResetHand`
  (`Actor.K2_DestroyActor` (`self.EquipedItem`))
  (bind _asbpa_survivor (cast `/Game/Animations/BPA_Survivor` (`SkeletalMeshComponent.GetAnimInstance` (`Character_Survivor.FPSMesh` (`self.MyCharacter`)))))
  (set `/Game/Animations/BPA_Survivor.WeaponBaseType` 0 _asbpa_survivor))

(fn `RightClickAction`)

(fn `SetInventoryMeshData`
  (`KismetArrayLibrary.Array_Clear` (`self.ItemMeshData`))
  (for _array_element (`self.Stocks`)
    (`KismetArrayLibrary.Array_AddUnique` (`self.ItemMeshData`) (make `/Game/Item/S_All_ItemMeshData` (break `/Game/Item/S_All_Item` _array_element) (`.Name_20_8969098149D6282D7AF70AB804D4FB00` (break `/Game/Item/S_All_Item` _array_element)) (`.NowStock_21_CB72561044233F9F4D0625899E384739` (break `/Game/Item/S_All_Item` _array_element))))))

(fn `ThrowItemFromInventory`
  (bind (_result _remainstock) (`self.RemoveItem` (`self.HandOnItemName`)))
  (if (and _result (== _remainstock 0))
    (`self.EmptyQuickSlot` (`self.EquippedSlot`))
    (set `self.HandOnItemName` "None")
    (`self.EquipOnHand` "None")))

(fn `ThrowTemporarilyItem`
  (set `self.HandOnItemName` "None")
  (`self.ResetHand`))

(fn `UseItem`)