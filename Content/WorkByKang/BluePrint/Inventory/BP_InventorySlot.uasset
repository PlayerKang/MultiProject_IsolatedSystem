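; BP_InventorySlot is a 3D inventory slot that displays one item type as up to five meshes.
; Its construction script reads the item's DT_Item row to set mesh scale and assign the mesh up to MaxStock.
; SetItemVisibilityByStock shows as many meshes as the current stock and prints a debug message.
; Hovering the cursor over a visible mesh, without clicking, passes the item name to the parent BP_InventoryMesh's SendAndCloseInventory.
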(event `self.ReceiveBeginPlay`)

(event `self.StaticMesh_0.OnBeginCursorOver`
  (params (TouchedComponent :type "PrimitiveComponent Object Reference"))
  (`self.EquipFromInventory` TouchedComponent))

(event `self.StaticMesh_1.OnBeginCursorOver`
  (params (TouchedComponent :type "PrimitiveComponent Object Reference"))
  (`self.EquipFromInventory` TouchedComponent))

(event `self.StaticMesh_2.OnBeginCursorOver`
  (params (TouchedComponent :type "PrimitiveComponent Object Reference"))
  (`self.EquipFromInventory` TouchedComponent))

(event `self.StaticMesh_3.OnBeginCursorOver`
  (params (TouchedComponent :type "PrimitiveComponent Object Reference"))
  (`self.EquipFromInventory` TouchedComponent))

(event `self.StaticMesh_4.OnBeginCursorOver`
  (params (TouchedComponent :type "PrimitiveComponent Object Reference"))
  (`self.EquipFromInventory` TouchedComponent))

(fn `BP_InventorySlot_Click`
  (params (Touched :type "MovieScenePrimitiveMaterialTrack Object Reference")))

(fn `EquipFromInventory`
  (params (TouchedComponent :type "SceneComponent Object Reference"))
  (bind _returnvalue (`self.GetParentActor`))
  (if (`SceneComponent.bVisible` TouchedComponent)
    (`/Engine/EditorBlueprintResources/StandardMacros.IsValid` _returnvalue
      (:`Is Valid`
        (bind _asbp_inventory_mesh (cast `/Game/WorkByKang/BluePrint/Inventory/BP_InventoryMesh` _returnvalue))
        (`/Game/WorkByKang/BluePrint/Inventory/BP_InventoryMesh.SendAndCloseInventory` _asbp_inventory_mesh (`self.ItemRawName`))))))

(fn `GetNumberFromMesh`
  (params (Object :type "Object Object Reference"))
  (returns (RightS :type String))
  (return (`.RightS` (`KismetStringLibrary.Split` (`KismetSystemLibrary.GetObjectName` Object) "_"))))

(fn `SetItemVisibilityByStock`
  (params (NowStock :type Integer))
  (bind _staticmesh_0 (`self.StaticMesh_0`))
  (`KismetSystemLibrary.PrintString` (`KismetStringLibrary.Concat_StrStr` (`KismetStringLibrary.Conv_NameToString` (`self.ItemRawName`)) " Stock : " (`KismetStringLibrary.Conv_IntToString` NowStock)) true true (struct :`R` 0.255187 :`B` 1.0 :`A` 1.0) 10.0)
  (switch `int` NowStock
    (:`0`
      (`SceneComponent.SetVisibility` _staticmesh_0 false false)
      (`SceneComponent.SetVisibility` (`self.StaticMesh_1`) false false)
      (`SceneComponent.SetVisibility` (`self.StaticMesh_2`) false false)
      (`SceneComponent.SetVisibility` (`self.StaticMesh_3`) false false)
      (`SceneComponent.SetVisibility` (`self.StaticMesh_4`) false false))
    (:`1`
      (`SceneComponent.SetVisibility` _staticmesh_0 true false)
      (`SceneComponent.SetVisibility` (`self.StaticMesh_1`) false false)
      (`SceneComponent.SetVisibility` (`self.StaticMesh_2`) false false)
      (`SceneComponent.SetVisibility` (`self.StaticMesh_3`) false false)
      (`SceneComponent.SetVisibility` (`self.StaticMesh_4`) false false))
    (:`2`
      (`SceneComponent.SetVisibility` _staticmesh_0 true false)
      (`SceneComponent.SetVisibility` (`self.StaticMesh_1`) true false)
      (`SceneComponent.SetVisibility` (`self.StaticMesh_2`) false false)
      (`SceneComponent.SetVisibility` (`self.StaticMesh_3`) false false)
      (`SceneComponent.SetVisibility` (`self.StaticMesh_4`) false false))
    (:`3`
      (`SceneComponent.SetVisibility` _staticmesh_0 true false)
      (`SceneComponent.SetVisibility` (`self.StaticMesh_1`) true false)
      (`SceneComponent.SetVisibility` (`self.StaticMesh_2`) true false)
      (`SceneComponent.SetVisibility` (`self.StaticMesh_3`) false false)
      (`SceneComponent.SetVisibility` (`self.StaticMesh_4`) false false))
    (:`4`
      (`SceneComponent.SetVisibility` _staticmesh_0 true false)
      (`SceneComponent.SetVisibility` (`self.StaticMesh_1`) true false)
      (`SceneComponent.SetVisibility` (`self.StaticMesh_2`) true false)
      (`SceneComponent.SetVisibility` (`self.StaticMesh_3`) true false)
      (`SceneComponent.SetVisibility` (`self.StaticMesh_4`) false false))
    (:`5`
      (`SceneComponent.SetVisibility` _staticmesh_0 true false)
      (`SceneComponent.SetVisibility` (`self.StaticMesh_1`) true false)
      (`SceneComponent.SetVisibility` (`self.StaticMesh_2`) true false)
      (`SceneComponent.SetVisibility` (`self.StaticMesh_3`) true false)
      (`SceneComponent.SetVisibility` (`self.StaticMesh_4`) true false))))

(fn `SetMeshByIndex`
  (params (NewMesh :type "StaticMesh Object Reference") (Index :type Integer))
  (switch `int` Index
    (:`0`
      (`StaticMeshComponent.SetStaticMesh` (`self.StaticMesh_0`) NewMesh))
    (:`1`
      (`StaticMeshComponent.SetStaticMesh` (`self.StaticMesh_1`) NewMesh))
    (:`2`
      (`StaticMeshComponent.SetStaticMesh` (`self.StaticMesh_2`) NewMesh))
    (:`3`
      (`StaticMeshComponent.SetStaticMesh` (`self.StaticMesh_3`) NewMesh))
    (:`4`
      (`StaticMeshComponent.SetStaticMesh` (`self.StaticMesh_4`) NewMesh))))

(fn `UserConstructionScript`
  (bind _returnvalue (`|GetDataTableRow` "/Game/Item/DT_Item.DT_Item" (`self.ItemRawName`))
    (:`then`
      (bind (_itemtype _name _maxstock _nowstock _mesh _handsizetransform) (break `/Game/Item/S_All_Item` _returnvalue))
      (`SceneComponent.SetWorldScale3D` (`self.StaticMesh_1`) (.scale _handsizetransform))
      (`SceneComponent.SetWorldScale3D` (`self.StaticMesh_2`) (.scale _handsizetransform))
      (`SceneComponent.SetWorldScale3D` (`self.StaticMesh_3`) (.scale _handsizetransform))
      (`SceneComponent.SetWorldScale3D` (`self.StaticMesh_4`) (.scale _handsizetransform))
      (`SceneComponent.SetWorldScale3D` (`self.StaticMesh_0`) (.scale _handsizetransform))
      (for _index (range _maxstock)
        (`self.SetMeshByIndex` _mesh _index)))))