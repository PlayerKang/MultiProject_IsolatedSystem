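; BP_RoomWindow is an interactive two-panel room window that extends a parent interactable, giving each panel its own trigger range and open state.
; On interaction input, whichever panel has the player in range plays a sound and toggles open or closed.
; Swing and slide flags select timeline-driven rotation or relative-location interpolation of each pivot.
; Input is ignored while either panel animates, and timelines reverse to close.
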(event `self.Trigger1.OnComponentBeginOverlap`
  (params (OverlappedComponent :type "PrimitiveComponent Object Reference") (OtherActor :type "Actor Object Reference") (OtherComp :type "PrimitiveComponent Object Reference") (OtherBodyIndex :type Integer) (bFromSweep :type Boolean) (SweepResult :type "HitResult Structure (by ref)"))
  (set `self.IsInAnotherRange` (== OtherActor (`GameplayStatics.GetPlayerPawn` 0))))

(event `self.ReceiveBeginPlay`
  (`parent.ReceiveBeginPlay`)
  (set `self.AnotherSourcePosition` (`SceneComponent.RelativeLocation` (`self.Pivot1`))))

(event `self.Trigger1.OnComponentEndOverlap`
  (params (OverlappedComponent :type "PrimitiveComponent Object Reference") (OtherActor :type "Actor Object Reference") (OtherComp :type "PrimitiveComponent Object Reference") (OtherBodyIndex :type Integer))
  (if (== OtherActor (`GameplayStatics.GetPlayerPawn` 0))
    (set `self.IsInAnotherRange` false)))

(event `/Game/WorkByKang/BluePrint/Interection/BPI_Interection.InterectionInput`
  (params (Character :type "Actor Object Reference"))
  (if (or (`self.IsInRange`) (`self.IsInAnotherRange`))
    (`self.DoorInteract`)))

(event `self.DoorInteract`
  (bind _sourceposition (`self.SourcePosition`))
  (bind _anothersourceposition (`self.AnotherSourcePosition`))
  (if (not (or (`self.IsAnimating`) (`self.IsAnotherAnimating`)))
    (`|ExecutionSequence`
      (:`then_0`
        (if (`self.IsSwingType`)
          (`|ExecutionSequence`
            (:`then_0`
              (if (`self.IsInRange`)
                (set `self.IsAnimating` true)
                (`self.PlaySound`)
                (if (`self.IsOpen`)
                  (bind (_direction _alpha) (`Timeline|타임라인` :!via `Reverse` :!label _label)
                    (:`Update`
                      (`SceneComponent.K2_SetRelativeRotation` (`self.Pivot`) (`KismetMathLibrary.RLerp` (struct) (`self.TargetRotation`) _alpha) false false))
                    (:`Finished`
                      (set `self.IsOpen` (not (`self.IsOpen`)))
                      (set `self.IsAnimating` false)))
                  (else
                    (goto _label)))))
            (:`then_1`
              (if (`self.IsInAnotherRange`)
                (set `self.IsAnotherAnimating` true)
                (`self.PlaySound`)
                (if (`self.IsAnotherOpen`)
                  (bind (_direction_2 _alpha_2) (`Timeline|타임라인_3` :!via `Reverse` :!label _label_2)
                    (:`Update`
                      (`SceneComponent.K2_SetRelativeRotation` (`self.Pivot1`) (`KismetMathLibrary.RLerp` (struct) (`self.AnotherTargetRotation`) _alpha_2) false false))
                    (:`Finished`
                      (set `self.IsAnotherOpen` (not (`self.IsAnotherOpen`)))
                      (set `self.IsAnotherAnimating` false)))
                  (else
                    (goto _label_2))))))))
      (:`then_1`
        (if (`self.IsSlideType`)
          (`|ExecutionSequence`
            (:`then_0`
              (if (`self.IsInRange`)
                (set `self.IsAnimating` true)
                (`self.PlaySound`)
                (if (`self.IsOpen`)
                  (bind (_direction_3 _alpha_3) (`Timeline|타임라인_0` :!via `Reverse` :!label _label_3)
                    (:`Update`
                      (`SceneComponent.K2_SetRelativeLocation` (`self.Pivot`) (`KismetMathLibrary.VLerp` _sourceposition (+ _sourceposition (`self.TargetPosition`)) _alpha_3) false false))
                    (:`Finished`
                      (set `self.IsOpen` (not (`self.IsOpen`)))
                      (set `self.IsAnimating` false)))
                  (else
                    (goto _label_3)))))
            (:`then_1`
              (if (`self.IsInAnotherRange`)
                (set `self.IsAnotherAnimating` true)
                (`self.PlaySound`)
                (if (`self.IsAnotherOpen`)
                  (bind (_direction_4 _alpha_4) (`Timeline|타임라인_1` :!via `Reverse` :!label _label_4)
                    (:`Update`
                      (`SceneComponent.K2_SetRelativeLocation` (`self.Pivot1`) (`KismetMathLibrary.VLerp` _anothersourceposition (+ _anothersourceposition (`self.AnotherTargetPosition`)) _alpha_4) false false))
                    (:`Finished`
                      (set `self.IsAnotherOpen` (not (`self.IsAnotherOpen`)))
                      (set `self.IsAnotherAnimating` false)))
                  (else
                    (goto _label_4)))))))))))

(fn `UserConstructionScript`
  (`parent.UserConstructionScript`))