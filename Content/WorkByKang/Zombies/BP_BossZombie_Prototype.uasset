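; Prototype boss zombie character that reacts to damage, can be killed, and supplies minimap icon data.
; Any damage stops the bite attack montage, then heavy single hits play a head hit reaction and lighter ones a right-arm reaction.
; When the head reaction completes, or the death montage from the interaction input blends out, movement is disabled and the mesh ragdolls.
; GetMapIconData returns location, yaw and the minimap component's icon settings.
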(event `self.ReceiveAnyDamage`
  (params (Damage :type "Float (single-precision)") (DamageType :type "DamageType Object Reference") (InstigatedBy :type "Controller Object Reference") (DamageCauser :type "Actor Object Reference"))
  (bind _mesh (`self.Mesh`))
  (bind _mesh_2 (`self.Mesh`))
  (if (> Damage 90.0)
    (`self.StopAnimMontage` "/Game/Zombie_old_ver/Ramin_Anim/BiteNeck_Start_Att_Montage.BiteNeck_Start_Att_Montage")
    (`|PlayMontage` _mesh "/Game/Zombie_old_ver/Ramin_Anim/RemainZombie_HitReact_Head_Montage.RemainZombie_HitReact_Head_Montage"
      (:`OnCompleted`
        (`CharacterMovementComponent.DisableMovement` (`self.CharacterMovement`))
        (`SkeletalMeshComponent.Stop` _mesh_2)
        (`PrimitiveComponent.SetSimulatePhysics` _mesh_2 true)))
    (else
      (`self.StopAnimMontage` "/Game/Zombie_old_ver/Ramin_Anim/BiteNeck_Start_Att_Montage.BiteNeck_Start_Att_Montage")
      (`|PlayMontage` _mesh "/Game/Zombie_old_ver/Ramin_Anim/RemainZombie_HitReact_RightArm_Montage.RemainZombie_HitReact_RightArm_Montage"))))

(event `/Game/WorkByKang/BluePrint/Interection/BPI_Interection.InterectionInput`
  (params (Character :type "Actor Object Reference"))
  (bind _mesh (`self.Mesh`))
  (`|PlayMontage` (`self.Mesh`) "/Game/Zombie_old_ver/NoHead_Anim/NoheadZombie_Idle_Death_Montage.NoheadZombie_Idle_Death_Montage"
    (:`OnBlendOut`
      (`CharacterMovementComponent.DisableMovement` (`self.CharacterMovement`))
      (`SkeletalMeshComponent.Stop` _mesh)
      (`PrimitiveComponent.SetSimulatePhysics` _mesh true))))

(fn `GetMapIconData`
  (returns (location :type "Vector Structure") (icon :type "Texture2D Object Reference") (`icon size` :type "Vector2D Structure") (Rotation_Yaw :type "Float (double-precision)"))
  (bind (_returnvalue_roll _returnvalue_pitch _returnvalue_yaw) (`KismetMathLibrary.BreakRotator` (`self.K2_GetActorRotation`)))
  (bind _minimap_icon_component (`self.Minimap_Icon_Component`))
  (return (`self.K2_GetActorLocation`) (`/PLG_Minimap/Minimap_Icon_Component.icon` _minimap_icon_component) (`/PLG_Minimap/Minimap_Icon_Component.Icon Size` _minimap_icon_component) _returnvalue_yaw))

(fn `UserConstructionScript`)