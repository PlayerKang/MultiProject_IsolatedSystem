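; BP_BlindZombie is a zombie character that reacts to interaction and point damage and appears on the minimap.
; Interaction plays a death montage, then on blend out disables movement, stops the mesh and enables physics simulation for a ragdoll.
; Point damage prints the hit bone and, for the Head, plays a left-arm hit reaction montage.
; GetMapIconData supplies location, yaw and the minimap component's icon settings.
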(event `/Game/WorkByKang/BluePrint/Interection/BPI_Interection.InterectionInput`
  (params (Character :type "Actor Object Reference"))
  (bind _mesh (`self.Mesh`))
  (`|PlayMontage` (`self.Mesh`) "/Game/Zombie_old_ver/Ramin_Anim/RemainZombie_Idle_Death_Montage.RemainZombie_Idle_Death_Montage"
    (:`OnBlendOut`
      (`CharacterMovementComponent.DisableMovement` (`self.CharacterMovement`))
      (`SkeletalMeshComponent.Stop` _mesh)
      (`PrimitiveComponent.SetSimulatePhysics` _mesh true))))

(event `self.ReceivePointDamage`
  (params (Damage :type "Float (single-precision)") (DamageType :type "DamageType Object Reference") (HitLocation :type "Vector Structure") (HitNormal :type "Vector Structure") (HitComponent :type "PrimitiveComponent Object Reference") (BoneName :type Name) (ShotFromDirection :type "Vector Structure") (InstigatedBy :type "Controller Object Reference") (DamageCauser :type "Actor Object Reference") (HitInfo :type "HitResult Structure (by ref)"))
  (`KismetSystemLibrary.PrintString` (`KismetStringLibrary.Conv_NameToString` BoneName))
  (switch `name` BoneName
    (:`head`
      (`|PlayMontage` (`self.Mesh`) "/Game/Zombie_old_ver/Ramin_Anim/RemainZombie_HitReact_LeftArm_Montage.RemainZombie_HitReact_LeftArm_Montage"))))

(fn `GetMapIconData`
  (returns (location :type "Vector Structure") (icon :type "Texture2D Object Reference") (`icon size` :type "Vector2D Structure") (Rotation_Yaw :type "Float (double-precision)"))
  (bind (_returnvalue_roll _returnvalue_pitch _returnvalue_yaw) (`KismetMathLibrary.BreakRotator` (`self.K2_GetActorRotation`)))
  (bind _minimap_icon_component (`self.Minimap_Icon_Component`))
  (return (`self.K2_GetActorLocation`) (`/PLG_Minimap/Minimap_Icon_Component.icon` _minimap_icon_component) (`/PLG_Minimap/Minimap_Icon_Component.Icon Size` _minimap_icon_component) _returnvalue_yaw))

(fn `UserConstructionScript`)