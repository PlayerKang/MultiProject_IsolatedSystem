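; Quest zombie enemy that attacks survivors and credits its killer's player state with a monster kill on death.
; Server-to-client attack events play standing or crawling montages, with notifies toggling a timed left-hand sphere trace that damages survivors; the right-hand trace is never started here.
; Point damage maps bones to hit reactions, disabled arms and body parts.
; Heavy hits hide the bone, spawn the part, and make leg-hit zombies crawl.
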(event `self.ReceiveBeginPlay`
  ;[1 1 1] 비긴플레이
  (`parent.ReceiveBeginPlay`))

(event `Attack On Server`
  ;[1 1 1] Attack 애니메이션 리플리케이션 완료!
  (`self.Attack On Client`))

(event `Attack On Client`
  ;[1 1 1] Attack 애니메이션 리플리케이션 완료!
  (if (`self.IsCrawl?`)
    (set `self.NonAttackableAnim` "/Game/Zombie_old_ver/Ramin_Anim/RemainZombie_Crawl_Idle_Search_Montage.RemainZombie_Crawl_Idle_Search_Montage")
    (set `self.AttackAnim` "/Game/Zombie_old_ver/Ramin_Anim/RemainZombie_Crawl_Attack01_Montage.RemainZombie_Crawl_Attack01_Montage")
    (else
      (set `self.NonAttackableAnim` "/Game/Zombie_old_ver/Ramin_Anim/RemainZombie_Idle_Search_Montage.RemainZombie_Idle_Search_Montage")
      (set `self.AttackAnim` "/Game/Zombie_old_ver/Ramin_Anim/RemainZombie_Attack03_Montage.RemainZombie_Attack03_Montage")))
  (if (or (`self.RightHandCanAttack?`) (`self.leftHandCanAttack?`))
    (`|PlayMontage` (`self.Mesh`) (`self.AttackAnim`) 1.0 0.0 "Default"
      (:`OnNotifyBegin`
        (`KismetSystemLibrary.K2_SetTimer` null "LeftHandSphereTrace" 0.05 true))
      (:`OnNotifyEnd`
        (`KismetSystemLibrary.K2_ClearTimer` null "LeftHandSphereTrace")
        (set `self.LeftTraceCheck` false)))
    (else
      (`|PlayMontage` (`self.Mesh`) (`self.NonAttackableAnim`) 1.0 0.0 "Default"))))

(event `self.ReceivePointDamage`
  (params (Damage :type "Float (single-precision)") (DamageType :type "DamageType Object Reference") (HitLocation :type "Vector Structure") (HitNormal :type "Vector Structure") (HitComponent :type "PrimitiveComponent Object Reference") (BoneName :type Name) (ShotFromDirection :type "Vector Structure") (InstigatedBy :type "Controller Object Reference") (DamageCauser :type "Actor Object Reference") (HitInfo :type "HitResult Structure (by ref)"))
  (bind _mesh (`self.Mesh`))
  (set `self.Damage` Damage)
  (set `self.KillingPlayer` InstigatedBy)
  (`|ExecutionSequence`
    (:`then_0`
      (`KismetSystemLibrary.PrintString` (`KismetStringLibrary.Conv_NameToString` BoneName))
      (bind _returnvalue (`SkinnedMeshComponent.IsBoneHiddenByName` _mesh (`SkinnedMeshComponent.GetParentBone` _mesh BoneName)))
      (bind _returnvalue_2 (`SkinnedMeshComponent.IsBoneHiddenByName` _mesh BoneName))
      (if (not (or _returnvalue_2 _returnvalue))
        (switch `name` BoneName
          (:`head`
            (set `self.Hide Bone Name` "head" :!label _label)
            (set `self.BodyPartName` "HeadPart")
            (set `self.HitReactAnimMontage` "/Game/Zombie_old_ver/Ramin_Anim/RemainZombie_HitReact_Head_Montage1.RemainZombie_HitReact_Head_Montage1" :!label _label_2))
          (:`neck_01`
            (goto _label))
          (:`pelvis`
            (set `self.Hide Bone Name` "None" :!label _label_3)
            (set `self.BodyPartName` "None")
            (goto _label_2))
          (:`spine_01`
            (goto _label_3))
          (:`spine_02`
            (goto _label_3))
          (:`spine_03`
            (goto _label_3))
          (:`clavicle_l`
            (set `self.Hide Bone Name` "upperarm_l" :!label _label_4)
            (set `self.BodyPartName` "ArmPart")
            (set `self.HitReactAnimMontage` "/Game/Zombie_old_ver/Ramin_Anim/RemainZombie_HitReact_LeftArm_Montage.RemainZombie_HitReact_LeftArm_Montage" :!label _label_5)
            (set `self.leftHandCanAttack?` false))
          (:`upperarm_l`
            (goto _label_4))
          (:`lowerarm_l`
            (set `self.Hide Bone Name` "lowerarm_l")
            (set `self.BodyPartName` "LowerArmPart")
            (goto _label_5))
          (:`hand_l`
            (set `self.Hide Bone Name` "hand_l")
            (set `self.BodyPartName` "HandPart")
            (goto _label_5))
          (:`clavicle_r`
            (set `self.Hide Bone Name` "upperarm_r" :!label _label_6)
            (set `self.BodyPartName` "ArmPart")
            (set `self.HitReactAnimMontage` "/Game/Zombie_old_ver/Ramin_Anim/RemainZombie_HitReact_RightArm_Montage1.RemainZombie_HitReact_RightArm_Montage1" :!label _label_7)
            (set `self.RightHandCanAttack?` false))
          (:`upperarm_r`
            (goto _label_6))
          (:`lowerarm_r`
            (set `self.Hide Bone Name` "lowerarm_r")
            (set `self.BodyPartName` "LowerArmPart")
            (goto _label_7))
          (:`hand_r`
            (set `self.Hide Bone Name` "hand_r")
            (set `self.BodyPartName` "HandPart")
            (goto _label_7))
          (:`thigh_l`
            (set `self.Hide Bone Name` "thigh_l")
            (set `self.BodyPartName` "LegPart")
            (set `self.HitReactAnimMontage` "/Game/Zombie_old_ver/Ramin_Anim/RemainZombie_HitReact_LeftLeg_Montage.RemainZombie_HitReact_LeftLeg_Montage" :!label _label_8)
            (set `self.LegAttacked` true :!label _label_9))
          (:`calf_l`
            (set `self.Hide Bone Name` "calf_l")
            (set `self.BodyPartName` "LowerLegPart")
            (goto _label_8))
          (:`foot_l`
            (set `self.Hide Bone Name` "foot_l")
            (set `self.BodyPartName` "FootPart" :!label _label_10)
            (set `self.HitReactAnimMontage` "/Game/Zombie_old_ver/Ramin_Anim/RemainZombie_HitReact_Legs_To_CrawlIdle_Montage.RemainZombie_HitReact_Legs_To_CrawlIdle_Montage")
            (goto _label_9))
          (:`thigh_r`
            (set `self.Hide Bone Name` "thigh_r")
            (set `self.BodyPartName` "LegPart")
            (set `self.HitReactAnimMontage` "/Game/Zombie_old_ver/Ramin_Anim/RemainZombie_HitReact_RightLeg_Montage.RemainZombie_HitReact_RightLeg_Montage" :!label _label_11)
            (goto _label_9))
          (:`calf_r`
            (set `self.Hide Bone Name` "calf_r")
            (set `self.BodyPartName` "LowerLegPart")
            (goto _label_11))
          (:`foot_r`
            (set `self.Hide Bone Name` "foot_r")
            (goto _label_10)))
        (if (not (not (`self.IsCrawl?`)))
          (set `self.HitReactAnimMontage` "/Game/Zombie_old_ver/Ramin_Anim/RemainZombie_Crawl_Back_Montage.RemainZombie_Crawl_Back_Montage"))
        (`|PlayMontage` (`self.Mesh`) (`self.HitReactAnimMontage`)
          (:`then`
            (if (>= (`self.Damage`) 100.0)
              (`self.HideBoneAndSpawnBodyPart` HitInfo)
              (if (`self.LegAttacked`)
                (set `self.IsCrawl?` true)))))))
    (:`then_1`
      (`self.UpdateHP` (`self.Damage`)))))

(fn `Death`
  (`parent.Death`)
  (bind _asbp_player_state_s (cast `/Game/MainBluePrints/BP_PlayerStateS` (`Controller.PlayerState` (`self.KillingPlayer`))))
  (`/Game/MainBluePrints/BP_PlayerStateS.Add Kill Monster` _asbp_player_state_s))

(fn `LeftHandSphereTrace`
  (bind _returnvalue (`SceneComponent.K2_GetComponentLocation` (`self.TopPoint_L`)))
  (bind (_outhit _returnvalue_2) (`KismetSystemLibrary.SphereTraceSingleForObjects` :`Start` _returnvalue :`End` (`SceneComponent.K2_GetComponentLocation` (`self.BottomPoint_L`)) :`Radius` 7.0 :`ObjectTypes` (`|MakeArray` "ObjectTypeQuery3" :!type "EObjectTypeQuery Enum") :`DrawDebugType` "ForDuration"))
  (if _returnvalue_2
    (if (not (`self.LeftTraceCheck`))
      (set `self.LeftTraceCheck` true)
      (bind (_bblockinghit _binitialoverlap _time _distance _location _impactpoint _normal _impactnormal _physmat _hitactor) (`GameplayStatics.BreakHitResult` _outhit))
      (`self.MakeNoise` 1.0 null _impactpoint)
      (`GameplayStatics.PlaySoundAtLocation` null (0.0 0.0 0.0) (struct) 1.0 1.0 0.0 null null null null)
      (bind _asbp_survivor (cast `/Game/MainBluePrints/BP_Survivor` _hitactor))
      (`GameplayStatics.SpawnEmitterAtLocation` "/Game/Realistic_Starter_VFX_Pack_Vol2/Particles/Blood/P_Blood_Splat_Cone.P_Blood_Splat_Cone" _returnvalue (`SceneComponent.K2_GetComponentRotation` (`Actor.RootComponent` _hitactor)) (0.4 0.4 0.4) true "AutoRelease")
      (`GameplayStatics.ApplyPointDamage` _asbp_survivor 100.0 _impactpoint _outhit))))

(fn `RightHandSphereTrace`
  (bind _returnvalue (`SceneComponent.K2_GetComponentLocation` (`self.TopPoint_R`)))
  (bind (_outhit _returnvalue_2) (`KismetSystemLibrary.SphereTraceSingleForObjects` :`Start` _returnvalue :`End` (`SceneComponent.K2_GetComponentLocation` (`self.BottomPoint_R`)) :`Radius` 7.0 :`ObjectTypes` (`|MakeArray` "ObjectTypeQuery3" "ObjectTypeQuery4" "ObjectTypeQuery2" :!type "EObjectTypeQuery Enum") :`DrawDebugType` "ForDuration"))
  (if _returnvalue_2
    (if (not (`self.LeftTraceCheck`))
      (set `self.LeftTraceCheck` true)
      (bind (_bblockinghit _binitialoverlap _time _distance _location _impactpoint _normal _impactnormal _physmat _hitactor) (`GameplayStatics.BreakHitResult` _outhit))
      (`self.MakeNoise` 1.0 null _impactpoint)
      (`GameplayStatics.PlaySoundAtLocation` null (0.0 0.0 0.0) (struct) 1.0 1.0 0.0 null null null null)
      (bind _asbp_survivor (cast `/Game/MainBluePrints/BP_Survivor` _hitactor))
      (`GameplayStatics.SpawnEmitterAtLocation` "/Game/Realistic_Starter_VFX_Pack_Vol2/Particles/Blood/P_Blood_Splat_Cone.P_Blood_Splat_Cone" _returnvalue (`SceneComponent.K2_GetComponentRotation` (`Actor.RootComponent` _hitactor)) (0.4 0.4 0.4) true "AutoRelease")
      (`GameplayStatics.ApplyPointDamage` _asbp_survivor 100.0 _impactpoint _outhit))))

(fn `UserConstructionScript`)