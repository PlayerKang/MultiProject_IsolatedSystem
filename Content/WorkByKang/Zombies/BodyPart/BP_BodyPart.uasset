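; A zombie body part item that simulates physics, can be picked up as a temporary inventory item and serves as a melee weapon.
; Construction swaps out the inherited Item component for the skeletal mesh, taking scale and mass from the DT_Item row.
; Left click starts a looping timer that sphere-traces between two mesh points, applying point damage to the first hit only.
; AnimStop clears the timer and re-arms the hit check; debug trace drawing is enabled.
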(event `self.ReceiveBeginPlay`
  (`PrimitiveComponent.SetSimulatePhysics` (`self.SkeletalMesh`) true))

(event `/Game/WorkByKang/BluePrint/Interection/BPI_Interection.InterectionInput`
  (params (Character :type "Actor Object Reference"))
  (`/Game/WorkByKang/BluePrint/Inventory/BPC_InventorySystem.PickUpTemporarilyItem` (`self.GetComponentByClass` Character "/Game/WorkByKang/BluePrint/Inventory/BPC_InventorySystem.BPC_InventorySystem_C") self))

(event `/Game/WorkByKang/BluePrint/Interection/BPI_Interection.LeftClickInput`
  (`KismetSystemLibrary.K2_SetTimer` null "SphereTraceLoopDamage" 0.05 true))

(event `/Game/WorkByKang/BluePrint/Interection/BPI_Interection.AnimStop`
  (`KismetSystemLibrary.K2_ClearTimer` null "SphereTraceLoopDamage")
  (set `self.TraceCheck` false))

(fn `SphereTraceLoopDamage`
  (bind (_outhit _returnvalue) (`KismetSystemLibrary.SphereTraceSingle` :`Start` (`SceneComponent.K2_GetComponentLocation` (`self.TopPoint_SK`)) :`End` (`SceneComponent.K2_GetComponentLocation` (`self.BottomPoint_SK`)) :`Radius` (`self.SphereTraceRadius`) :`TraceChannel` "TraceTypeQuery1" :`DrawDebugType` "ForDuration" :`DrawTime` 10.0))
  (if _returnvalue
    (if (not (`self.TraceCheck`))
      (set `self.TraceCheck` true)
      (bind (_bblockinghit _binitialoverlap _time _distance _location _impactpoint _normal _impactnormal _physmat _hitactor) (`GameplayStatics.BreakHitResult` _outhit))
      (`GameplayStatics.ApplyPointDamage` _hitactor (`self.Damage`) _impactpoint _outhit))))

(fn `UserConstructionScript`
  (bind _skeletalmesh (`self.SkeletalMesh`))
  (bind _returnvalue (`|GetDataTableRow` "/Game/Item/DT_Item.DT_Item" (`self.ItemRowName`))
    (:`then`
      (`ActorComponent.K2_DestroyComponent` (`self.Item`))
      (bind (_itemtype _name _maxstock _nowstock _mesh _handsizetransform _baseanimtype _mass) (break `/Game/Item/S_All_Item` _returnvalue))
      (`SceneComponent.SetWorldScale3D` _skeletalmesh (.scale _handsizetransform))
      (`PrimitiveComponent.SetMassOverrideInKg` _skeletalmesh "None" _mass true))))