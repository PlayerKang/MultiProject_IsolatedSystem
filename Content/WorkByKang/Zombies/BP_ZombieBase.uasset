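; Base zombie character with health, AI-driven attacks, limb dismemberment and corpse burning.
; UpdateHP clamps health and triggers a ragdoll death, after which interaction sets the body on fire and later destroys it.
; Attack montages play when the blackboard AIState is Battle; hits are reported as touch events.
; Dismemberment hides a bone and spawns a DT_Item body part told which child segments were already missing; hidden bones are tracked for restoration.
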(event `self.ReceiveBeginPlay`
  (set `self.CurrentHP` (`self.MaxHP`)))

(event `/Game/WorkByKang/BluePrint/Interection/BPI_Interection.InterectionInput`
  (params (Character :type "Actor Object Reference"))
  (bind _mesh (`self.Mesh`))
  (if (`self.IsDeath?`)
    (bind _returnvalue (`GameplayStatics.SpawnEmitterAtLocation` "/Game/Realistic_Starter_VFX_Pack_Vol2/Particles/Fire/P_Fire_Big.P_Fire_Big" (`SceneComponent.K2_GetComponentLocation` _mesh) (`SceneComponent.K2_GetComponentRotation` _mesh) (0.3 0.3 0.3)))
    (`KismetSystemLibrary.Delay` 20.0)
    (`ActorComponent.K2_DestroyComponent` _returnvalue)
    (`self.K2_DestroyActor`)))

(event `Restore Departed Body Bones`
  (for _array_element (`self.HiddenBones`)
    (`SkinnedMeshComponent.UnHideBoneByName` (`self.Mesh`) _array_element)))

(event `self.ReceiveHit`
  (params (MyComp :type "PrimitiveComponent Object Reference") (Other :type "Actor Object Reference") (OtherComp :type "PrimitiveComponent Object Reference") (bSelfMoved :type Boolean) (HitLocation :type "Vector Structure") (HitNormal :type "Vector Structure") (NormalImpulse :type "Vector Structure") (Hit :type "HitResult Structure (by ref)"))
  (`AISense_Touch.ReportTouchEvent` self Other HitLocation) ; UE5 이상에서만 쓸  있음
)

(fn `Death`
  (bind _mesh (`self.Mesh`))
  (`CharacterMovementComponent.DisableMovement` (`self.CharacterMovement`))
  (`SkeletalMeshComponent.Stop` _mesh)
  (`PrimitiveComponent.SetSimulatePhysics` _mesh true)
  (set `self.IsDeath?` true))

(fn `GetPartHidden`
  (params (BoneName :type Name))
  (returns (BodyPartHidden :type "/Game/WorkByKang/Zombies/BodyPart/E_BodyPartHidden Enum"))
  (switch `name` BoneName
    (:`Default`
      (return "NewEnumerator2"))
    (:`clavicle_l`
      _)
    (:`upperarm_l`
      _)
    (:`lowerarm_l`
      (bind _returnvalue (`SkinnedMeshComponent.IsBoneHiddenByName` (`self.Mesh`) "hand_l"))
      (if _returnvalue
        (return "NewEnumerator0")
        (else
          (return "NewEnumerator2"))))
    (:`clavicle_r`
      (bind _returnvalue_2 (`SkinnedMeshComponent.IsBoneHiddenByName` (`self.Mesh`) "lowerarm_r" :!label _label))
      (if _returnvalue_2
        (return "NewEnumerator1")
        (else
          (bind _returnvalue_3 (`SkinnedMeshComponent.IsBoneHiddenByName` (`self.Mesh`) "hand_r"))
          (if _returnvalue_3
            (return "NewEnumerator0")
            (else
              (return "NewEnumerator2"))))))
    (:`upperarm_r`
      (goto _label))
    (:`lowerarm_r`
      (bind _returnvalue_4 (`SkinnedMeshComponent.IsBoneHiddenByName` (`self.Mesh`) "hand_r"))
      (if _returnvalue_4
        (return "NewEnumerator0")
        (else
          (return "NewEnumerator2"))))
    (:`thigh_l`
      (bind _returnvalue_5 (`SkinnedMeshComponent.IsBoneHiddenByName` (`self.Mesh`) "calf_l"))
      (if _returnvalue_5
        (return "NewEnumerator1")
        (else
          (bind _returnvalue_6 (`SkinnedMeshComponent.IsBoneHiddenByName` (`self.Mesh`) "foot_l"))
          (if _returnvalue_6
            (return "NewEnumerator0")
            (else
              (return "NewEnumerator2"))))))
    (:`calf_l`
      (bind _returnvalue_7 (`SkinnedMeshComponent.IsBoneHiddenByName` (`self.Mesh`) "foot_l"))
      (if _returnvalue_7
        (return "NewEnumerator0")
        (else
          (return "NewEnumerator2"))))
    (:`thigh_r`
      (bind _returnvalue_8 (`SkinnedMeshComponent.IsBoneHiddenByName` (`self.Mesh`) "calf_r"))
      (if _returnvalue_8
        (return "NewEnumerator1")
        (else
          (bind _returnvalue_9 (`SkinnedMeshComponent.IsBoneHiddenByName` (`self.Mesh`) "foot_r"))
          (if _returnvalue_9
            (return "NewEnumerator0")
            (else
              (return "NewEnumerator2"))))))
    (:`calf_r`
      (bind _returnvalue_10 (`SkinnedMeshComponent.IsBoneHiddenByName` (`self.Mesh`) "foot_r"))
      (if _returnvalue_10
        (return "NewEnumerator0")
        (else
          (return "NewEnumerator2")))))
  (bind _returnvalue_11 (`SkinnedMeshComponent.IsBoneHiddenByName` (`self.Mesh`) "lowerarm_l"))
  (if _returnvalue_11
    (return "NewEnumerator1")
    (else
      (bind _returnvalue_12 (`SkinnedMeshComponent.IsBoneHiddenByName` (`self.Mesh`) "hand_l"))
      (if _returnvalue_12
        (return "NewEnumerator0")
        (else
          (return "NewEnumerator2"))))))

(fn `HideBoneAndSpawnBodyPart`
  (params (Hit :type "HitResult Structure (by ref)"))
  (bind (_bblockinghit _binitialoverlap _time _distance _location _impactpoint _normal) (`GameplayStatics.BreakHitResult` Hit))
  (bind _bodypartname (`self.BodyPartName`))
  (bind _hide_bone_name (`self.Hide Bone Name`))
  (bind _returnvalue (`|GetDataTableRow` "/Game/Item/DT_Item.DT_Item" _bodypartname)
    (:`then`
      (`|SpawnActorFromClass` (`.BP_47_757DA67542F38347E47E3D9A8BD1682F` (break `/Game/Item/S_All_Item` _returnvalue)) (`KismetMathLibrary.MakeTransform` _location (`KismetMathLibrary.Conv_VectorToRotator` _normal)) "Undefined" "OverrideRootScale" null _bodypartname (`self.GetPartHidden` (`self.Hide Bone Name`)) null)
      (`KismetArrayLibrary.Array_AddUnique` (`self.HiddenBones`) _hide_bone_name)
      (`SkinnedMeshComponent.HideBoneByName` (`self.Mesh`) _hide_bone_name "PBO_None"))))

(fn `UpdateAttackAnimMontage`
  (bind _output_get (set `self.AIState` (cast `/Game/WorkByKim/AI/PatrolNPC/EN_AIState` (`BlackboardComponent.GetValueAsEnum` (`AIBlueprintHelperLibrary.GetBlackboard` (`self.GetController`)) "AIState"))))
  (switch `/Game/WorkByKim/AI/PatrolNPC/EN_AIState` _output_get
    (:`NewEnumerator2`
      (if (not (`self.IsAttacking`))
        (`self.PlayAnimMontage` (`self.AttackAnim`) 1.0 "Attack")))))

(fn `UpdateHP`
  (params (Change :type "Float (double-precision)"))
  (bind _returnvalue (- (`self.CurrentHP`) Change))
  (bind _returnvalue_2 (> _returnvalue 0.0))
  (if (and _returnvalue_2 (<= _returnvalue (`self.MaxHP`)))
    (set `self.CurrentHP` _returnvalue)
    (elif _returnvalue_2
      (set `self.CurrentHP` (`self.MaxHP`))
      (else
        (`self.Death`)))))

(fn `UserConstructionScript`)