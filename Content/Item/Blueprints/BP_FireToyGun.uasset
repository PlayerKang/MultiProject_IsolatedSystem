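; BP_FireToyGun is a toy gun item Blueprint that shoots a cosmetic flamethrower effect.
; Left-click input attaches the P_Flamethrower particle emitter to the Item component, using the Arrow component's relative transform, and stores it as FlameComponent.
; AnimStop calls the parent handler, then destroys that flame component after a short delay.
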(event `/Game/WorkByKang/BluePrint/Interection/BPI_Interection.LeftClickInput`
  (bind _arrow (`self.Arrow`))
  (bind _returnvalue (`GameplayStatics.SpawnEmitterAttached` "/Game/Realistic_Starter_VFX_Pack_Vol2/Particles/Fire/P_flamethrower.P_Flamethrower" (`self.Item`) "None" (`SceneComponent.RelativeLocation` _arrow) (`SceneComponent.RelativeRotation` _arrow)))
  (set `self.FlameComponent` _returnvalue))

(event `/Game/WorkByKang/BluePrint/Interection/BPI_Interection.AnimStop`
  (`parent.AnimStop`)
  (`KismetSystemLibrary.Delay` 3.0)
  (`ActorComponent.K2_DestroyComponent` (`self.FlameComponent`)))

(fn `UserConstructionScript`
  (`parent.UserConstructionScript`))