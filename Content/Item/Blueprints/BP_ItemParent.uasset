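; BP_ItemParent is a physics-simulated item that characters pick up through BPC_InventorySystem and can swing as a melee weapon.
; Construction looks up ItemRowName in DT_Item to set mesh, scale and mass.
; Left or right click starts a looping timer that sphere-traces from TopPoint to BottomPoint with debug drawing.
; TraceCheck limits point damage to the first hit until AnimStop clears the timer and resets it.
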(event `self.ReceiveBeginPlay`
  (`PrimitiveComponent.SetSimulatePhysics` (`self.Item`) true))

(event `/Game/WorkByKang/BluePrint/Interection/BPI_Interection.InterectionInput`
  (params (Character :type "Actor Object Reference"))
  (`/Game/WorkByKang/BluePrint/Inventory/BPC_InventorySystem.Pick Up Item` (`self.GetComponentByClass` Character "/Game/WorkByKang/BluePrint/Inventory/BPC_InventorySystem.BPC_InventorySystem_C") self))

(event `/Game/WorkByKang/BluePrint/Interection/BPI_Interection.LeftClickInput`
  (`KismetSystemLibrary.K2_SetTimer` null "SphereTraceLoop" 0.05 true))

(event `/Game/WorkByKang/BluePrint/Interection/BPI_Interection.AnimStop`
  (`KismetSystemLibrary.K2_ClearTimer` null "SphereTraceLoop")
  (set `self.TraceCheck` false))

(event `/Game/WorkByKang/BluePrint/Interection/BPI_Interection.RightClickInput`
  (`KismetSystemLibrary.K2_SetTimer` null "SphereTraceLoop" 0.05 true))

(fn `SphereTraceLoop`
  (bind (_outhit _returnvalue) (`KismetSystemLibrary.SphereTraceSingle` :`Start` (`SceneComponent.K2_GetComponentLocation` (`self.TopPoint`)) :`End` (`SceneComponent.K2_GetComponentLocation` (`self.BottomPoint`)) :`Radius` 5.0 :`TraceChannel` "TraceTypeQuery1" :`DrawDebugType` "ForDuration" :`DrawTime` 10.0))
  (if _returnvalue
    (if (not (`self.TraceCheck`))
      (set `self.TraceCheck` true)
      (bind (_bblockinghit _binitialoverlap _time _distance _location _impactpoint _normal _impactnormal _physmat _hitactor) (`GameplayStatics.BreakHitResult` _outhit))
      (`GameplayStatics.ApplyPointDamage` _hitactor 100.0 _impactpoint _outhit))))

(fn `UserConstructionScript`
  (bind _item (`self.Item`))
  (bind _returnvalue (`|GetDataTableRow` "/Game/Item/DT_Item.DT_Item" (`self.ItemRowName`))
    (:`then`
      (bind (_itemtype _name _maxstock _nowstock _mesh _handsizetransform _baseanimtype _mass) (break `/Game/Item/S_All_Item` _returnvalue))
      (`StaticMeshComponent.SetStaticMesh` _item _mesh)
      (`SceneComponent.SetWorldScale3D` _item (.scale _handsizetransform))
      (`PrimitiveComponent.SetMassOverrideInKg` _item "None" _mass true))))