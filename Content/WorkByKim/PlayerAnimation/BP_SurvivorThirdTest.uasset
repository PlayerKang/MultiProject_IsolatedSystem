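; Test player survivor character with crouch, sprint, map toggle, a hit-reaction blood overlay and minimap icon data.
; Each tick picks an idle, walk or run camera shake from speed and sphere-traces from the first-person camera for BPI_Interection actors, toggling a dot widget.
; The interact input plays a pickup montage whose notify messages the traced actor.
; Starting a sprint also reports noise at the player's location.
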(event `self.ReceiveBeginPlay`
  ;[1 1 1] Dot Widget
  (bind _returnvalue (`|CreateWidget` "/Game/Widgets/InterectDot.InterectDot_C"))
  (set `self.InterectDot` _returnvalue)
  (bind _returnvalue_2 (`|CreateWidget` "/Game/Widgets/BloodEffect.BloodEffect_C"))
  (`UserWidget.AddToViewport` _returnvalue_2 0)
  (set `self.WBP_Hud` _returnvalue_2))

(event `EnhancedInput|/Game/Input/Movement/IA_Crouching`
  (params (ActionValue :type Boolean) (ElapsedSeconds :type "Float (double-precision)") (TriggeredSeconds :type "Float (double-precision)") (InputAction :type "InputAction Object Reference" :default "/Game/Input/Movement/IA_Crouching.IA_Crouching"))
  ;[1 1 1] Crouch
  (:`Started`
    (`self.Crouch`))
  (:`Completed`
    (`self.UnCrouch`)))

(event `self.ReceiveTick`
  (params (DeltaSeconds :type "Float (single-precision)"))
  (bind _fpscameracomponent (`self.FPSCameraComponent`))
  (bind _interectdot (`self.InterectDot`))
  (bind _returnvalue (`SceneComponent.K2_GetComponentLocation` _fpscameracomponent))
  (bind _returnvalue_2 (`Widget.IsInViewport` _interectdot))
  (`|ExecutionSequence`
    (:`then_0`
      (`self.CameraShake`))
    (:`then_1`
      ;[1 1 1] Set HitActor for Dot Widget
      (set `self.HitActor` null)
      (`self.InterectDot`
        (:`then`
          (bind (_outhit _returnvalue_3) (`KismetSystemLibrary.SphereTraceSingle` _returnvalue (+ _returnvalue (* (`SceneComponent.GetForwardVector` _fpscameracomponent) 350.0)) 10.0 "TraceTypeQuery2" false (`|MakeArray` (`/Game/WorkByKang/BluePrint/Inventory/BPC_InventorySystem.EquipedItem` (`self.BPC_InventorySystem`)) :!type "Actor Object Reference")))
          (if _returnvalue_3
            (bind (_bblockinghit _binitialoverlap _time _distance _location _impactpoint _normal _impactnormal _physmat _hitactor) (`GameplayStatics.BreakHitResult` _outhit))
            (if (`KismetSystemLibrary.DoesImplementInterface` _hitactor "/Game/WorkByKang/BluePrint/Interection/BPI_Interection.BPI_Interection_C")
              (set `self.HitActor` _hitactor)
              (if (not _returnvalue_2)
                (`UserWidget.AddToViewport` _interectdot 0))
              (else
                (if _returnvalue_2 :!label _label
                  (`/Game/Widgets/InterectDot.Remove` _interectdot))))
            (else
              (goto _label))))
        (:`else`)))))

(event `EnhancedInput|/Game/Input/Movement/IA_Run`
  (params (ActionValue :type Boolean) (ElapsedSeconds :type "Float (double-precision)") (TriggeredSeconds :type "Float (double-precision)") (InputAction :type "InputAction Object Reference" :default "/Game/Input/Movement/IA_Run.IA_Run"))
  (bind _charactermovement (`self.CharacterMovement`))
  ;[1 1 1] Sprint
  (:`Started`
    (set `CharacterMovementComponent.MaxWalkSpeed` 300.0 _charactermovement)
    (`AISense_Hearing.ReportNoiseEvent` (`self.K2_GetActorLocation`) 1.0 (`GameplayStatics.GetPlayerPawn` 0)))
  (:`Completed`
    (set `CharacterMovementComponent.MaxWalkSpeed` 180.0 _charactermovement)))

(event `EnhancedInput|/Game/Input/Interface/IA_F_Interection`
  (params (ActionValue :type Boolean) (ElapsedSeconds :type "Float (double-precision)") (TriggeredSeconds :type "Float (double-precision)") (InputAction :type "InputAction Object Reference" :default "/Game/Input/Interface/IA_F_Interection.IA_F_Interection"))
  ;[1 1 1] Interection Input
  (:`Triggered`
    (bind _hitactor (`self.HitActor`)
      (:`then`
        (`|PlayMontage` (`self.FPSMesh`) "/Game/ArmsMeleeFPSAndBonusTemplate/MeleePACK/brassknuckles/anims/Anim_PickUpItem_Montage.Anim_PickUpItem_Montage" 0.4 0.0 "None"
          (:`OnNotifyBegin`
            (message `/Game/WorkByKang/BluePrint/Interection/BPI_Interection.InterectionInput` _hitactor self))))
      (:`else`))))

(event `self.ReceivePointDamage`
  (params (Damage :type "Float (single-precision)") (DamageType :type "DamageType Object Reference") (HitLocation :type "Vector Structure") (HitNormal :type "Vector Structure") (HitComponent :type "PrimitiveComponent Object Reference") (BoneName :type Name) (ShotFromDirection :type "Vector Structure") (InstigatedBy :type "Controller Object Reference") (DamageCauser :type "Actor Object Reference") (HitInfo :type "HitResult Structure (by ref)"))
  (`/Game/Widgets/BloodEffect.Play Attacked Anim` (`self.WBP_Hud`)))

(event `EnhancedInput|/Game/Input/Interface/IA_M_Map`
  (params (ActionValue :type Boolean) (ElapsedSeconds :type "Float (double-precision)") (TriggeredSeconds :type "Float (double-precision)") (InputAction :type "InputAction Object Reference" :default "/Game/Input/Interface/IA_M_Map.IA_M_Map"))
  (bind _returnvalue (`PlayerController.GetHUD` (`GameplayStatics.GetPlayerController` 0)))
  (:`Started`
    (`/Engine/EditorBlueprintResources/StandardMacros.FlipFlop`
      (:`A`
        (message `/PLG_Minimap/BPI_Minimap.ToggleMap` _returnvalue true))
      (:`B`
        (message `/PLG_Minimap/BPI_Minimap.ToggleMap` _returnvalue false)))))

(fn `CameraShake`
  (bind _returnvalue (`GameplayStatics.GetPlayerController` 0))
  (if (<= (`KismetMathLibrary.VSize` (`self.GetVelocity`)) 0.0)
    (`PlayerController.ClientStartCameraShake` :`self` _returnvalue :`Shake` "/Game/WorkByKang/BluePrint/CameraSetting/BP_CameraShakeIdle.BP_CameraShakeIdle_C")
    (elif (>= (`KismetMathLibrary.VSize` (`self.GetVelocity`)) 181.0)
      (`PlayerController.ClientStartCameraShake` :`self` _returnvalue :`Shake` "/Game/WorkByKang/BluePrint/CameraSetting/BP_CameraShakeRun.BP_CameraShakeRun_C")
      (else
        (`PlayerController.ClientStartCameraShake` :`self` _returnvalue :`Shake` "/Game/WorkByKang/BluePrint/CameraSetting/BP_CameraShakeWalk.BP_CameraShakeWalk_C")))))

(fn `GetMapIconData`
  (returns (location :type "Vector Structure") (icon :type "Texture2D Object Reference") (`icon size` :type "Vector2D Structure") (Rotation_Yaw :type "Float (double-precision)"))
  (bind (_returnvalue_roll _returnvalue_pitch _returnvalue_yaw) (`KismetMathLibrary.BreakRotator` (`self.K2_GetActorRotation`)))
  (bind _minimap_icon_component (`self.Minimap_Icon_Component`))
  (return (`self.K2_GetActorLocation`) (`/PLG_Minimap/Minimap_Icon_Component.icon` _minimap_icon_component) (`/PLG_Minimap/Minimap_Icon_Component.Icon Size` _minimap_icon_component) _returnvalue_yaw))

(fn `UserConstructionScript`)