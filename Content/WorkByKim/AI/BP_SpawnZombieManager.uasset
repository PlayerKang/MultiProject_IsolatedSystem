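; BP_SpawnZombieManager keeps the level's population of BP_ResponeBlindZombie at its starting count.
; Shortly after BeginPlay it records how many of those zombies exist and caches all SpawnPoint actors.
; On Tick it accumulates time and, at each CountCheck interval, recounts them, spawning one replacement at a random spawn point if the count has dropped and printing a debug message.
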(event `self.ReceiveBeginPlay`
  (`KismetSystemLibrary.Delay` 3.0)
  (bind _outactors (`GameplayStatics.GetAllActorsOfClass` "/Game/WorkByKim/AI/BP_ResponeBlindZombie.BP_ResponeBlindZombie_C"))
  (set `self.InitZombieCount` (`KismetMathLibrary.Conv_IntToDouble` (`KismetArrayLibrary.Array_Length` _outactors)))
  (bind _outactors_2 (`GameplayStatics.GetAllActorsOfClass` "/Game/WorkByKim/AI/SpawnPoint.SpawnPoint_C"))
  (set `self.SpawnPoints` _outactors_2)
  (set `self.IsInitCheck` true))

(event `self.ReceiveTick`
  (params (DeltaSeconds :type "Float (single-precision)"))
  (if (`self.IsInitCheck`)
    (set `self.DeltaTime` (+ DeltaSeconds (`self.DeltaTime`)))
    (if (>= (`self.DeltaTime`) (`self.Count Check`))
      (set `self.DeltaTime` 0.0)
      (bind _outactors (`GameplayStatics.GetAllActorsOfClass` "/Game/WorkByKim/AI/BP_ResponeBlindZombie.BP_ResponeBlindZombie_C"))
      (if (< (`KismetArrayLibrary.Array_Length` _outactors) (`self.InitZombieCount`))
        (`|SpawnActorFromClass` "/Game/WorkByKim/AI/BP_ResponeBlindZombie.BP_ResponeBlindZombie_C" (`KismetMathLibrary.MakeTransform` (`self.K2_GetActorLocation` (`KismetArrayLibrary.Array_Random` (`self.SpawnPoints`)))) "AdjustIfPossibleButDontSpawnIfColliding" "OverrideRootScale" null null)
        (`KismetSystemLibrary.PrintString` "스폰좀비")))))

(fn `UserConstructionScript`)