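; BP_NewNPC is an AI-controlled NPC that plays an attack montage while in battle and reports physical hits as touch events.
; Hit events feed ReportTouchEvent with the other actor and hit location, using a UE5 touch-sense call.
; UpdateAttackAnimMontage reads the AIState enum from the controller's Blackboard and plays the attack montage in Battle unless IsAttacking is set.
; EventMontageFinish clears IsAttacking, which this graph never sets to true.
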(event `self.ReceiveHit`
  (params (MyComp :type "PrimitiveComponent Object Reference") (Other :type "Actor Object Reference") (OtherComp :type "PrimitiveComponent Object Reference") (bSelfMoved :type Boolean) (HitLocation :type "Vector Structure") (HitNormal :type "Vector Structure") (NormalImpulse :type "Vector Structure") (Hit :type "HitResult Structure (by ref)"))
  ;[0.476 0.476 0.476] Hit하면 Touch이벤트 발생
  (`AISense_Touch.ReportTouchEvent` self Other HitLocation) ; UE5 이상에서만 쓸  있음
)

(fn `EventMontageFinish`
  (set `self.IsAttacking` false))

(fn `UpdateAttackAnimMontage`
  (bind _output_get (set `self.AIState` (cast `/Game/WorkByKim/AI/PatrolNPC/EN_AIState` (`BlackboardComponent.GetValueAsEnum` (`AIBlueprintHelperLibrary.GetBlackboard` (`self.GetController`)) "AIState"))))
  (switch `/Game/WorkByKim/AI/PatrolNPC/EN_AIState` _output_get
    (:`NewEnumerator2`
      (if (not (`self.IsAttacking`))
        (`self.PlayAnimMontage` "/Game/WorkByKim/AI/NewNPC/Animation/AM_NewNPCAttack.AM_NewNPCAttack" 1.0 "Attack")))))

(fn `UserConstructionScript`)