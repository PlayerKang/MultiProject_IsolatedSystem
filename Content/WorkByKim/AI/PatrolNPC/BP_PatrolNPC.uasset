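; BP_PatrolNPC is a zombie NPC whose melee attack damages BP_Survivor.
; Attack picks montages by crawl state, playing the attack if either hand can attack, otherwise a search idle.
; Montage notifies start and stop a looping timer that sphere-traces pawns between two left-hand points.
; A TraceCheck flag limits each swing to one hit, which makes noise and, on a survivor, spawns blood and applies point damage.
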(event `Attack`
  (if (`self.IsCrawl?`)
    (set `self.NonAttackableAnim_0` "/Game/Zombie_old_ver/NoHead_Anim/NH_Zombie_Crawl_Idle_Search_Montage.NH_Zombie_Crawl_Idle_Search_Montage")
    (set `self.AttackAnim` "/Game/WorkByKim/AI/PatrolNPC/Animation/AM_Attack.AM_Attack")
    (else
      (set `self.NonAttackableAnim_0` "/Game/Zombie_old_ver/NoHead_Anim/NH_Zombie_Idle_Search_Montage.NH_Zombie_Idle_Search_Montage")
      (set `self.AttackAnim` "/Game/Zombie_old_ver/NoHead_Anim/NH_Zombie_Crawl_Attack01_Montage.NH_Zombie_Crawl_Attack01_Montage")))
  (if (or (`self.RightHandCanAttack?`) (`self.leftHandCanAttack?`))
    (`|PlayMontage` (`self.Mesh`) (`self.AttackAnim`)
      (:`OnNotifyBegin`
        (`KismetSystemLibrary.K2_SetTimer` null "LeftHandSphereTrace" 0.05 true))
      (:`OnNotifyEnd`
        (`KismetSystemLibrary.K2_ClearTimer` null "LeftHandSphereTrace")
        (set `self.TraceCheck` false)))
    (else
      (`|PlayMontage` (`self.Mesh`) (`self.NonAttackableAnim_0`)))))

(fn `LeftHandSphereTrace`
  (bind _returnvalue (`SceneComponent.K2_GetComponentLocation` (`self.TopPoint_L`)))
  (bind (_outhit _returnvalue_2) (`KismetSystemLibrary.SphereTraceSingleForObjects` :`Start` _returnvalue :`End` (`SceneComponent.K2_GetComponentLocation` (`self.BottomPoint_L`)) :`Radius` 7.0 :`ObjectTypes` (`|MakeArray` "ObjectTypeQuery3" :!type "EObjectTypeQuery Enum") :`DrawDebugType` "ForDuration"))
  (if _returnvalue_2
    (if (not (`self.TraceCheck`))
      (set `self.TraceCheck` true)
      (bind (_bblockinghit _binitialoverlap _time _distance _location _impactpoint _normal _impactnormal _physmat _hitactor) (`GameplayStatics.BreakHitResult` _outhit))
      (`self.MakeNoise` 1.0 null _impactpoint)
      (`GameplayStatics.PlaySoundAtLocation` null (0.0 0.0 0.0) (struct) 1.0 1.0 0.0 null null null null)
      (bind _asbp_survivor (cast `/Game/MainBluePrints/BP_Survivor` _hitactor))
      (`GameplayStatics.SpawnEmitterAtLocation` "/Game/Realistic_Starter_VFX_Pack_Vol2/Particles/Blood/P_Blood_Splat_Cone.P_Blood_Splat_Cone" _returnvalue (`SceneComponent.K2_GetComponentRotation` (`Actor.RootComponent` _hitactor)) (0.4 0.4 0.4) true "AutoRelease")
      (`GameplayStatics.ApplyPointDamage` _asbp_survivor 100.0 _impactpoint _outhit))))

(fn `UserConstructionScript`)