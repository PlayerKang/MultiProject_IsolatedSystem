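; AI controller for NPCs that runs the BT_NewNPC behavior tree on BeginPlay and reacts to sounds through AI Perception.
; When a hearing stimulus arrives and the Zombie tag check fails, it writes the sound location as a vector to the TargetActor blackboard key and changes the AIState enum.
; Other senses are ignored, and the touch handler is an empty stub.
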(event `self.ReceiveBeginPlay`
  ;[1 0.2238 0.8693] BT_NormalNPC 실행
  (`self.RunBehaviorTree` "/Game/WorkByKim/AI/NewNPC/BT_NewNPC.BT_NewNPC"))

(event `self.AIPerception.OnTargetPerceptionUpdated`
  (params (Actor :type "Actor Object Reference") (Stimulus :type "AIStimulus Structure"))
  ;[0.9676 0.3571 1] AI Perception - Hearing / Touch
  (`self.HandleSoundSense` Stimulus))

(fn `HandleSoundSense`
  (params (Stimulus :type "AIStimulus Structure"))
  (bind _blackboard (`self.Blackboard`))
  (bind _returnvalue (`AIPerceptionSystem.GetSenseClassForStimulus` Stimulus))
  (if (== _returnvalue "/Script/AIModule.AISense_Hearing")
    (if (not (`self.ActorHasTag` "Zombie"))
      (`BlackboardComponent.SetValueAsVector` _blackboard "TargetActor" (`.StimulusLocation` (break `AIStimulus` (`local.Stimulus`))))
      (`BlackboardComponent.SetValueAsEnum` _blackboard "AIState" (enumliteral `/Game/WorkByKim/AI/PatrolNPC/EN_AIState` "NewEnumerator1")))
    (else
      (return))))

(fn `HandleTouchEvent`)

(fn `UserConstructionScript`)