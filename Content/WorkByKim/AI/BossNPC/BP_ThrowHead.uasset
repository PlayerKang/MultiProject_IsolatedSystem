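; BP_ThrowHead is a boss NPC actor, by its name a thrown head, that damages survivors on contact.
; From BeginPlay, a looping timer runs a debug-drawn sphere trace for pawns between its TopPoint and BottomPoint.
; The first hit clears the timer, makes noise and calls a sound at world origin.
; If the pawn is a BP_Survivor, it also spawns blood and applies point damage.
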(event `self.ReceiveBeginPlay`
  (`KismetSystemLibrary.K2_SetTimer` null "HeadSphereTrace" 0.05 true))

(event `TraceEnd`
  (`KismetSystemLibrary.K2_ClearTimer` null "HeadSphereTrace"))

(fn `HeadSphereTrace`
  (bind _returnvalue (`SceneComponent.K2_GetComponentLocation` (`self.TopPoint`)))
  (bind (_outhit _returnvalue_2) (`KismetSystemLibrary.SphereTraceSingleForObjects` :`Start` _returnvalue :`End` (`SceneComponent.K2_GetComponentLocation` (`self.BottomPoint`)) :`Radius` 22.0 :`ObjectTypes` (`|MakeArray` "ObjectTypeQuery3" :!type "EObjectTypeQuery Enum") :`DrawDebugType` "ForDuration"))
  (if _returnvalue_2
    (`self.TraceEnd`)
    (if (not (`self.TraceCheck`))
      (set `self.TraceCheck` true)
      (bind (_bblockinghit _binitialoverlap _time _distance _location _impactpoint _normal _impactnormal _physmat _hitactor) (`GameplayStatics.BreakHitResult` _outhit))
      (`self.MakeNoise` 1.0 null _impactpoint)
      (`GameplayStatics.PlaySoundAtLocation` null (0.0 0.0 0.0) (struct) 1.0 1.0 0.0 null null null null)
      (bind _asbp_survivor (cast `/Game/MainBluePrints/BP_Survivor` _hitactor))
      (`GameplayStatics.SpawnEmitterAtLocation` "/Game/Realistic_Starter_VFX_Pack_Vol2/Particles/Blood/P_Blood_Splat_Cone.P_Blood_Splat_Cone" _returnvalue (`SceneComponent.K2_GetComponentRotation` (`Actor.RootComponent` _hitactor)) (0.4 0.4 0.4) true "AutoRelease")
      (`GameplayStatics.ApplyPointDamage` _asbp_survivor 100.0 _impactpoint _outhit))))

(fn `UserConstructionScript`)