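; Boss NPC character Blueprint that handles the AI boss's attack animation, touch sensing and minimap icon data.
; Hits are forwarded as touch events, with the boss as the receiver.
; The attack update reads AIState from the blackboard and plays the RightAttack montage section in Battle when IsAttacking is false; montage finish clears that flag.
; GetMapIconData returns location, yaw and the minimap component's icon settings.
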(event `self.ReceiveHit`
  (params (MyComp :type "PrimitiveComponent Object Reference") (Other :type "Actor Object Reference") (OtherComp :type "PrimitiveComponent Object Reference") (bSelfMoved :type Boolean) (HitLocation :type "Vector Structure") (HitNormal :type "Vector Structure") (NormalImpulse :type "Vector Structure") (Hit :type "HitResult Structure (by ref)"))
  ;[0.3499 0.4325 0.476] Hit하면 Touch이벤트 발생
  (`AISense_Touch.ReportTouchEvent` self Other HitLocation) ; UE5 이상에서만 쓸  있음
)

(fn `EventMontageFinish`
  (`KismetSystemLibrary.PrintString` "BossNPC attack anim finish!")
  (set `self.IsAttacking` false))

(fn `GetMapIconData`
  (returns (location :type "Vector Structure") (icon :type "Texture2D Object Reference") (`icon size` :type "Vector2D Structure") (Rotation_Yaw :type "Float (double-precision)"))
  (bind (_returnvalue_roll _returnvalue_pitch _returnvalue_yaw) (`KismetMathLibrary.BreakRotator` (`self.K2_GetActorRotation`)))
  (bind _minimap_icon_component (`self.Minimap_Icon_Component`))
  (return (`self.K2_GetActorLocation`) (`/PLG_Minimap/Minimap_Icon_Component.icon` _minimap_icon_component) (`/PLG_Minimap/Minimap_Icon_Component.Icon Size` _minimap_icon_component) _returnvalue_yaw))

(fn `UpdateAttackAnimMontage`
  (bind _output_get (set `self.AIState` (cast `/Game/WorkByKim/AI/PatrolNPC/EN_AIState` (`BlackboardComponent.GetValueAsEnum` (`AIBlueprintHelperLibrary.GetBlackboard` (`self.GetController`)) "AIState"))))
  (switch `/Game/WorkByKim/AI/PatrolNPC/EN_AIState` _output_get
    (:`NewEnumerator2`
      (if (not (`self.IsAttacking`))
        (`KismetSystemLibrary.PrintString` "BossNPC is Attacking player")
        (`self.PlayAnimMontage` "/Game/WorkByKim/AI/PatrolNPC/Animation/AM_Attack.AM_Attack" 1.0 "RightAttack") ; 애님수정예정
      ))))

(fn `UserConstructionScript`)