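; BP_InventoryMesh is an actor that holds a Stocks item list, apparently intended as a mesh representation of the survivor's inventory.
; On BeginPlay it loops over Stocks and switches on item type, but no case does anything yet.
; When destroyed, it writes Stocks back to the player BP_Survivor's inventory system component.
; AddItem and RemoveItem are stubs, with RemoveItem always returning false.
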(event `self.ReceiveBeginPlay`
  ;[1 1 1] Initialize / Save Inventory
  (`self.SetInventoryMesh`))

(event `self.ReceiveDestroyed`
  ;[1 1 1] Initialize / Save Inventory
  (`self.SaveInventoryChange`))

(fn `AddItem`
  (params (Item :type "/Game/Item/S_All_Item Structure"))
  (returns (Result :type Boolean)))

(fn `RemoveItem`
  (params (Item :type "/Game/Item/S_All_Item Structure"))
  (returns (Result :type Boolean))
  (return false))

(fn `SaveInventoryChange`
  (bind _asbp_survivor (cast `/Game/BluePrint/BP_Survivor` (`GameplayStatics.GetPlayerPawn` 0)))
  (set `/Game/BluePrint/Inventory/BPC_InventorySystem.Stocks` (`self.Stocks`) (`/Game/BluePrint/BP_Survivor.BPC_InventorySystem` _asbp_survivor)))

(fn `SetInventoryMesh`
  (for _array_element (`self.Stocks`)
    (switch `/Game/Item/E_ItemType` (`.ItemType_2_A8FA9B8F4C75B31A39A6C5BE21F09EAC` (break `/Game/Item/S_All_Item` _array_element)))))

(fn `UserConstructionScript`)