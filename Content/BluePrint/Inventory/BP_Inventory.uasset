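; BP_Inventory is an in-world inventory display Blueprint with clickable slot components for combining, a banana and gauze.
; Clicking the banana or gauze ground hides that item's component and prints its name, while the combine ground only prints a debug message.
; A loop over the Stocks array is never executed, and SetInventoryInfo and the construction script are empty stubs.
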(event `self.CombineGrounnd.OnClicked`
  (params (TouchedComponent :type "PrimitiveComponent Object Reference") (ButtonPressed :type "Key Structure"))
  (`KismetSystemLibrary.PrintString` "combine"))

(event `self.Banana_Ground.OnClicked`
  (params (TouchedComponent :type "PrimitiveComponent Object Reference") (ButtonPressed :type "Key Structure"))
  (`KismetSystemLibrary.PrintString` "Banana")
  (`SceneComponent.SetVisibility` (`self.Banana`) false false))

(event `self.Gauze_Ground.OnClicked`
  (params (TouchedComponent :type "PrimitiveComponent Object Reference") (ButtonPressed :type "Key Structure"))
  (`KismetSystemLibrary.PrintString` "Gauze")
  (`SceneComponent.SetVisibility` (`self.Gauze`) false false))

(fn `SetInventoryInfo`)

(fn `UserConstructionScript`)