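; BPC_InventorySystem is an inventory component that stores items in Stocks and shows them as a spawned in-world mesh actor.
; ShowInventory spawns a scaled-down BP_InventoryMesh at the BP_Survivor's InventoryPoint and passes it Stocks; CloseInventory destroys it.
; AddItem appends to Stocks, leaving its stack-limit check unconnected.
; RemoveItem only returns false, and the combine and quick-slot functions are empty stubs.
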(fn `AddItem`
  (params (Item :type "/Game/Item/S_All_Item Structure"))
  (returns (Result :type Boolean))
  (`KismetArrayLibrary.Array_Add` (`self.Stocks`) Item))

(fn `AddQuikslot`)

(fn `ClickCombineItem`)

(fn `CloseInventory`
  (`Actor.K2_DestroyActor` (`self.SpawnedInventory`)))

(fn `EmptyQuickSlot`)

(fn `RemoveItem`
  (params (Item :type "/Game/Item/S_All_Item Structure"))
  (returns (Result :type Boolean))
  (return false))

(fn `ShowInventory`
  (bind _asbp_survivor (cast `/Game/BluePrint/BP_Survivor` (`GameplayStatics.GetPlayerPawn` 0)))
  (bind (_returnvalue_location _returnvalue_rotation) (`KismetMathLibrary.BreakTransform` (`SceneComponent.K2_GetComponentToWorld` (`/Game/BluePrint/BP_Survivor.InventoryPoint` _asbp_survivor))))
  (bind _returnvalue (`|SpawnActorFromClass` "/Game/BluePrint/Inventory/BP_InventoryMesh.BP_InventoryMesh_C" (`KismetMathLibrary.MakeTransform` _returnvalue_location _returnvalue_rotation (0.03 0.03 0.03)) "Undefined" "OverrideRootScale" null (`self.Stocks`) null))
  (set `self.SpawnedInventory` _returnvalue))