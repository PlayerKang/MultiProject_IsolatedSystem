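; BP_Zombie is a zombie character Blueprint that reacts to incoming damage with hit animations or death.
; Any hit stops the neck-bite attack montage, then plays a head or right-arm hit-react montage depending on whether that single hit exceeds a damage threshold.
; When the head reaction completes, movement is disabled and the mesh switches to physics simulation as a ragdoll.
; No health is tracked between hits.
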(event `self.ReceiveAnyDamage`
  (params (Damage :type "Float (single-precision)") (DamageType :type "DamageType Object Reference") (InstigatedBy :type "Controller Object Reference") (DamageCauser :type "Actor Object Reference"))
  (bind _mesh (`self.Mesh`))
  (bind _mesh_2 (`self.Mesh`))
  (if (> Damage 90.0)
    (`self.StopAnimMontage` "/Game/Zombie_old_ver/Ramin_Anim/BiteNeck_Start_Att_Montage.BiteNeck_Start_Att_Montage")
    (`|PlayMontage` _mesh_2 "/Game/Zombie_old_ver/Ramin_Anim/RemainZombie_HitReact_Head_Montage.RemainZombie_HitReact_Head_Montage"
      (:`OnCompleted`
        (`CharacterMovementComponent.DisableMovement` (`self.CharacterMovement`))
        (`SkeletalMeshComponent.Stop` _mesh)
        (`PrimitiveComponent.SetSimulatePhysics` _mesh true)))
    (else
      (`self.StopAnimMontage` "/Game/Zombie_old_ver/Ramin_Anim/BiteNeck_Start_Att_Montage.BiteNeck_Start_Att_Montage")
      (`|PlayMontage` _mesh_2 "/Game/Zombie_old_ver/Ramin_Anim/RemainZombie_HitReact_RightArm_Montage.RemainZombie_HitReact_RightArm_Montage"))))

(fn `UserConstructionScript`)