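; Zombie AI controller that runs the BT_Zombie behavior tree on possess and feeds it player detection from AI Perception.
; Sensing an actor tagged Player cancels the lose-target timer and sets HasLineofSight and EnemyActor on the Blackboard.
; Any other perception update starts a one-shot timer that clears both keys when it expires, giving a grace period before the zombie forgets its target.
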(event `self.ReceivePossess`
  (params (PossessedPawn :type "Pawn Object Reference"))
  (`self.RunBehaviorTree` "/Game/Zombie_old_ver/BT_Zombie.BT_Zombie"))

(event `self.AIPerception.OnTargetPerceptionUpdated`
  (params (Actor :type "Actor Object Reference") (Stimulus :type "AIStimulus Structure"))
  (bind _blackboard (`self.Blackboard`))
  ;[1 1 1] 4초 안에 캐릭터를 발견하면  따라다녀라
  (if (and (`self.ActorHasTag` Actor "Player") (`.bSuccessfullySensed` (break `AIStimulus` Stimulus)))
    (`KismetSystemLibrary.K2_ClearAndInvalidateTimerHandle` (`self.Timer`))
    (`BlackboardComponent.SetValueAsBool` _blackboard (`self.hasLineofSight`) true)
    (`BlackboardComponent.SetValueAsObject` _blackboard (`self.EnemyActor`) Actor)
    (else
      (bind _returnvalue (`KismetSystemLibrary.K2_SetTimerDelegate` (delegate `EndTimer`) (`self.Time`)))
      (set `self.Timer` _returnvalue))))

(event `EndTimer`
  (bind _blackboard (`self.Blackboard`))
  ;[1 1 1] 4초 안에 캐릭터를 발견하면  따라다녀라
  (`BlackboardComponent.SetValueAsBool` _blackboard (`self.hasLineofSight`) false)
  (`BlackboardComponent.SetValueAsObject` _blackboard (`self.EnemyActor`) null))

(event `self.ReceiveAnyDamage`
  (params (Damage :type "Float (single-precision)") (DamageType :type "DamageType Object Reference") (InstigatedBy :type "Controller Object Reference") (DamageCauser :type "Actor Object Reference")))

(fn `UserConstructionScript`)