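; Basement HUD Blueprint that creates the HUD widget on BeginPlay, gives its minimap a BlackCircle brush and sets game-only input.
; Binds to the local BP_PlayerStateS for health and stamina updates, retrying by timer until the PlayerState is valid.
; BindPlayerState hooks any given player's name, kill and death dispatchers to refresh the player list.
; Tick writes player location and normalized yaw into the MP_Minimap parameter collection.
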(event `self.ReceiveBeginPlay`
  (bind _returnvalue (`GameplayStatics.GetPlayerController` 0))
  (bind _returnvalue_2 (`|CreateWidget` "/Game/WorkByLGH/HudWidget.HudWidget_C"))
  (bind _output_get (set `self.WBP_HudWidget` _returnvalue_2))
  (`UserWidget.AddToViewport` _output_get 0)
  (`Image.SetBrushFromTexture` (`/Game/WorkByLGH/HudWidget.Minimap` _returnvalue_2) "/Game/WorkByLGH/BlackCircle.BlackCircle" true)
  (`self.BindMyPlayerState`)
  (`WidgetBlueprintLibrary.SetInputMode_GameOnly` _returnvalue)
  (set `PlayerController.bShowMouseCursor` false _returnvalue))

(event `self.ReceiveTick`
  (params (DeltaSeconds :type "Float (single-precision)"))
  (bind _returnvalue (`GameplayStatics.GetPlayerCharacter` 0))
  (bind _yaw (.yaw (`self.K2_GetActorRotation` _returnvalue)))
  (`KismetMaterialLibrary.SetVectorParameterValue` "/PLG_Minimap/UI_Assets/MP_Minimap.MP_Minimap" "PlayerLocation" (`KismetMathLibrary.Conv_VectorToLinearColor` (`self.K2_GetActorLocation` _returnvalue)))
  (`KismetMaterialLibrary.SetScalarParameterValue` "/PLG_Minimap/UI_Assets/MP_Minimap.MP_Minimap" "PlayerYaw" (/ (`KismetMathLibrary.SelectFloat` (+ _yaw 360.0) _yaw (< _yaw 0.0)) 360.0)))

(fn `BindMyPlayerState`
  (bind _playerstate (`Controller.PlayerState` (`GameplayStatics.GetPlayerController` 0)))
  (`/Engine/EditorBlueprintResources/StandardMacros.IsValid` _playerstate
    (:`Is Valid`
      (bind _asbp_player_state_s (cast `/Game/MainBluePrints/BP_PlayerStateS` _playerstate))
      (add `/Game/MainBluePrints/BP_PlayerStateS.EvDispather_UpdateHealth` _asbp_player_state_s (`|CreateDelegate` :!event `UpdateHealth`))
      (add `/Game/MainBluePrints/BP_PlayerStateS.EvDispather_UpdateStamina` _asbp_player_state_s (`|CreateDelegate` :!event `UpdateStamina`))
      (`self.UpdateHealth` (`/Game/MainBluePrints/BP_PlayerStateS.CurrentHealth` _asbp_player_state_s) (`/Game/MainBluePrints/BP_PlayerStateS.MaxHealth` _asbp_player_state_s))
      (`self.UpdateStamina` (`/Game/MainBluePrints/BP_PlayerStateS.CurrentStamina` _asbp_player_state_s) (`/Game/MainBluePrints/BP_PlayerStateS.MaxStamina` _asbp_player_state_s)))
    (:`Is Not Valid`
      (`KismetSystemLibrary.K2_SetTimer` null "BindMyPlayerState" 0.1))))

(fn `BindPlayerState`
  (params (PlayerState :type "/Game/MainBluePrints/BP_PlayerStateS Object Reference"))
  (add `/Game/MainBluePrints/BP_PlayerStateS.EvDispather_ChangeName` PlayerState (`|CreateDelegate` :!event `EventChangePlayerName`))
  (add `/Game/MainBluePrints/BP_PlayerStateS.EvDispather_KillMonster` PlayerState (`|CreateDelegate` :!event `EventChangeKill`))
  (add `/Game/MainBluePrints/BP_PlayerStateS.EvDispather_Death` PlayerState (`|CreateDelegate` :!event `EventChangeDeath`)))

(fn `EventChangeDeath`
  (params (Death :type Integer))
  (`self.UpdatePlayerListHUD`))

(fn `EventChangeKill`
  (params (KillMonster :type Integer))
  (`self.UpdatePlayerListHUD`))

(fn `EventChangePlayerName`
  (params (PlayerName :type String))
  (`self.UpdatePlayerListHUD`))

(fn `TempUpdate`
  (bind _wbp_hudwidget (`self.WBP_HudWidget`))
  (`/Engine/EditorBlueprintResources/StandardMacros.IsValid` (`self.WBP_HudWidget`)
    (:`Is Valid`
      (bind _asbp_player_state_s (cast `/Game/MainBluePrints/BP_PlayerStateS` (`Controller.PlayerState` (`GameplayStatics.GetPlayerController` 0))))
      (`/Game/WorkByLGH/HudWidget.UpdateHealth` _wbp_hudwidget (`/Game/MainBluePrints/BP_PlayerStateS.CurrentHealth` _asbp_player_state_s) (`/Game/MainBluePrints/BP_PlayerStateS.MaxHealth` _asbp_player_state_s))
      (`/Game/WorkByLGH/HudWidget.UpdateStamina` _wbp_hudwidget (`/Game/MainBluePrints/BP_PlayerStateS.CurrentStamina` _asbp_player_state_s) (`/Game/MainBluePrints/BP_PlayerStateS.MaxStamina` _asbp_player_state_s)))
    (:`Is Not Valid`
      (`KismetSystemLibrary.K2_SetTimer` null "TempUpdate"))))

(fn `UpdateHealth`
  (params (CurrentHealth :type "Float (double-precision)") (MaxHealth :type "Float (double-precision)"))
  (bind _wbp_hudwidget (`self.WBP_HudWidget`))
  (`/Engine/EditorBlueprintResources/StandardMacros.IsValid` _wbp_hudwidget
    (:`Is Valid`
      (`/Game/WorkByLGH/HudWidget.UpdateHealth` _wbp_hudwidget CurrentHealth MaxHealth))))

(fn `UpdatePlayerListHUD`
  (bind _wbp_hudwidget (`self.WBP_HudWidget`))
  (`/Engine/EditorBlueprintResources/StandardMacros.IsValid` _wbp_hudwidget
    (:`Is Valid`
      (`/Game/WorkByLGH/HudWidget.UpdatePlayerList` _wbp_hudwidget))
    (:`Is Not Valid`
      (`KismetSystemLibrary.K2_SetTimer` null "UpdatePlayerListHUD" 0.1))))

(fn `UpdateStamina`
  (params (CurrentSprint :type "Float (double-precision)") (MaxSprint :type "Float (double-precision)"))
  (bind _wbp_hudwidget (`self.WBP_HudWidget`))
  (`/Engine/EditorBlueprintResources/StandardMacros.IsValid` _wbp_hudwidget
    (:`Is Valid`
      (`/Game/WorkByLGH/HudWidget.UpdateStamina` _wbp_hudwidget CurrentSprint MaxSprint))))

(fn `UserConstructionScript`)