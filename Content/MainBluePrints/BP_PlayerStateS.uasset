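; BP_PlayerStateS is a player state holding name, health, stamina and hunger, plus kill and death values.
; BeginPlay fills health and stamina to max and binds the state to BP_HudS on player controller 0.
; Name, health and stamina RepNotifies fire event dispatchers, while heal and recovery functions clamp their values to max.
; Hunger initialization assigns itself, and the update functions and remaining RepNotifies have no effect.
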(event `self.ReceiveBeginPlay`
  (set `self.CurrentHealth` (`self.MaxHealth`))
  (set `self.CurrentStamina` (`self.MaxStamina`))
  (set `self.CurrentHunger` (`self.CurrentHunger`))
  (bind _asbp_hud_s (cast `/Game/MainBluePrints/BP_HudS` (`PlayerController.GetHUD` (`GameplayStatics.GetPlayerController` 0))))
  (`/Game/MainBluePrints/BP_HudS.BindPlayerState` _asbp_hud_s self))

(fn `Add Heal`
  (params (Heal :type "Float (double-precision)"))
  (set `self.CurrentHealth` (`KismetMathLibrary.FClamp` (+ (`self.CurrentHealth`) Heal) 0.0 (`self.MaxHealth`))))

(fn `Add Recorvery`
  (params (Recorvery :type "Float (double-precision)"))
  (set `self.CurrentStamina` (`KismetMathLibrary.FClamp` (+ (`self.CurrentStamina`) Recorvery) 0.0 (`self.MaxStamina`))))

(fn `OnRep_CurrentHealth`
  (`self.EvDispather_UpdateHealth` (`self.CurrentHealth`) (`self.MaxHealth`)))

(fn `OnRep_CurrentStamina`
  (`self.EvDispather_UpdateStamina` (`self.CurrentStamina`) (`self.MaxStamina`)))

(fn `OnRep_Death`)

(fn `OnRep_KillMonster`)

(fn `OnRep_MaxHealth`)

(fn `OnRep_strPlayerName`
  (`self.EvDispather_ChangeName` (`self.strPlayerName`)))

(fn `UpdateHealth`
  (if (<= (`self.CurrentHealth`) 0.0)
    _))

(fn `UpdateStamina`)

(fn `UserConstructionScript`)