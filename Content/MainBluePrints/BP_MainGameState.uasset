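; BP_MainGameState is a game state Blueprint that drives the boss fight UI.
; BossBattle creates and shows a WBP_BossHpBar, and Tick keeps its bar synced to the clamped ratio of BossCurrentHP to BossMaxHP while the widget is valid.
; BossDeath adds a WBP_PlayerKillBoss widget to the viewport and plays its fade-out.
; The graph never changes the boss HP values, only reads them.
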(event `BossBattle`
  (bind _returnvalue (`|CreateWidget` "/Game/WorkByKim/AI/Widget/WBP_BossHpBar.WBP_BossHpBar_C"))
  (bind _output_get (set `self.Boss HP Bar Widget` _returnvalue))
  (`ProgressBar.SetPercent` (`/Game/WorkByKim/AI/Widget/WBP_BossHpBar.HealthBar_Boss` _output_get) (/ (`self.BossCurrentHP`) (`self.BossMaxHP`)))
  (`UserWidget.AddToViewport` _output_get 0)
  (`Widget.SetVisibility` _output_get "Visible"))

(event `self.ReceiveTick`
  (params (DeltaSeconds :type "Float (single-precision)"))
  (bind _boss_hp_bar_widget (`self.Boss HP Bar Widget`)
    (:`then`
      (`ProgressBar.SetPercent` (`/Game/WorkByKim/AI/Widget/WBP_BossHpBar.HealthBar_Boss` _boss_hp_bar_widget) (`KismetMathLibrary.FClamp` (/ (`self.BossCurrentHP`) (`self.BossMaxHP`)))))
    (:`else`)))

(event `BossDeath`
  (bind _returnvalue (`|CreateWidget` "/Game/WorkByKang/BluePrint/Quest/WBP_PlayerKillBoss.WBP_PlayerKillBoss_C"))
  (`UserWidget.AddToViewport` _returnvalue 0)
  (`/Game/WorkByKang/BluePrint/Quest/WBP_PlayerKillBoss.Play FadeOut` _returnvalue))

(fn `UserConstructionScript`)